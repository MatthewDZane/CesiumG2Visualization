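; Networked controller that loads a Netbox snapshot of regions, sites and locations for every BP_G2_Topology actor.
; Refresh starts a token-based request; on snapshot update the server spawns linked Netbox actors and passes them to each topology.
; A looping server timer multicasts those actors; clients set up once all maps are set, refreshing their own snapshot if needed.
; Helpers send Netbox PATCH requests; CreateDevices is defined but not called here.
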(event `Refresh SERVER`
  (`self.Reset Load Flags MULTICAST`)
  (`self.Refresh`))

(event `Reset Load Flags MULTICAST`
  (set `self.Snapshot Loaded` false)
  (set `self.Snapshot Load Started` false)
  (bind _outactors (`GameplayStatics.GetAllActorsOfClass` "/CesiumG2Visualization/BP_G2_Topology.BP_G2_Topology_C"))
  (for _array_element _outactors
    (set `/CesiumG2Visualization/BP_G2_Topology.Snapshot Setup Started` false _array_element)))

(event `self.ReceiveBeginPlay`
  (`/Engine/EditorBlueprintResources/ActorMacros.Switch Has Authority`
    (:`Authority`
      (`self.Refresh`))))

(event `self.OnSnapshotUpdate`
  (set `self.Snapshot Load Started` false)
  (set `self.Snapshot Loaded` true)
  (`/Engine/EditorBlueprintResources/ActorMacros.Switch Has Authority`
    (:`Authority`
      (bind _outactors (`GameplayStatics.GetAllActorsOfClass` "/CesiumG2Visualization/BP_G2_Topology.BP_G2_Topology_C"))
      (for _array_element _outactors
        (`/CesiumG2Visualization/BP_G2_Topology.Clear Visualization` _array_element)
        (bind (_created_regions _created_sites _created_locations) (`self.Create Replicated Actors` _array_element))
        (`/CesiumG2Visualization/BP_G2_Topology.Set Replicated Actor Maps` _array_element _created_regions _created_sites _created_locations))
      (`KismetSystemLibrary.K2_SetTimerDelegate` (delegate `Check Clients Snapshot`) 20.0 true 10.0))
    (:`Remote`
      (bind _outactors_2 (`GameplayStatics.GetAllActorsOfClass` "/CesiumG2Visualization/BP_G2_Topology.BP_G2_Topology_C"))
      (for _array_element_2 _outactors_2
        (`/CesiumG2Visualization/BP_G2_Topology.Setup Snapshot` _array_element_2)))))

(event `Check Clients Snapshot`
  (`KismetSystemLibrary.PrintString` "Checking")
  (bind _outactors (`GameplayStatics.GetAllActorsOfClass` "/CesiumG2Visualization/BP_G2_Topology.BP_G2_Topology_C"))
  (for _array_element _outactors
    (bind _snapshot (`/CesiumG2Visualization/BP_G2_Topology.Snapshot` _array_element))
    (bind _values (`BlueprintMapLibrary.Map_Values` (`/CesiumG2Visualization/BP_G2_Snapshot.Name to Region Map` _snapshot)))
    (bind _values_2 (`BlueprintMapLibrary.Map_Values` (`/CesiumG2Visualization/BP_G2_Snapshot.Name to Site Map` _snapshot)))
    (bind _values_3 (`BlueprintMapLibrary.Map_Values` (`/CesiumG2Visualization/BP_G2_Snapshot.Name to Location Map` _snapshot)))
    (`self.Set G2 Topology Replicated Actor Maps MULTICAST` _array_element _values _values_2 _values_3)))

(event `Set G2 Topology Replicated Actor Maps MULTICAST`
  (params (`G2 Topology` :type "/CesiumG2Visualization/BP_G2_Topology Object Reference") (Regions :type "Array of /CesiumG2Visualization/G2VisualizationActors/NetBoxActors/BP_Netbox_Region Object Reference (by ref)") (Sites :type "Array of /CesiumG2Visualization/G2VisualizationActors/NetBoxActors/BP_Netbox_Site Object Reference (by ref)") (Locations :type "Array of /CesiumG2Visualization/G2VisualizationActors/NetBoxActors/BP_Netbox_Location Object Reference (by ref)"))
  (if (not (`/CesiumG2Visualization/BP_G2_Topology.Snapshot Setup Started` `G2 Topology`))
    (`/CesiumG2Visualization/BP_G2_Topology.Set Replicated Actor Maps` `G2 Topology` Regions Sites Locations)
    (bind _result (`self.All Replicated Actors Set`))
    (if _result
      (if (`self.Snapshot Loaded`)
        (`/CesiumG2Visualization/BP_G2_Topology.Setup Snapshot` `G2 Topology`)
        (elif (not (`self.Snapshot Load Started`))
          (`KismetSystemLibrary.PrintString` "Refreshing")
          (`self.Refresh`))))))

(fn `All Replicated Actors Set`
  (returns (Result :type Boolean))
  (bind _outactors (`GameplayStatics.GetAllActorsOfClass` "/CesiumG2Visualization/BP_G2_Topology.BP_G2_Topology_C"))
  (for _array_element _outactors
    (if (or (not (`/CesiumG2Visualization/BP_G2_Topology.Name to Region Map Set` _array_element)) (not (`/CesiumG2Visualization/BP_G2_Topology.Name to Site Map Set` _array_element)) (not (`/CesiumG2Visualization/BP_G2_Topology.Name To Location Map Set` _array_element)))
      (return false)))
  (return true))

(fn `Create Devices`
  (params (`Name to Site Map` :type "Map of String to /CesiumG2Visualization/G2VisualizationActors/NetBoxActors/BP_Netbox_Site Object Reference") (`Name to Location Map` :type "Map of String to /CesiumG2Visualization/G2VisualizationActors/NetBoxActors/BP_Netbox_Location Object Reference") (`G2 Topology` :type "/CesiumG2Visualization/BP_G2_Topology Object Reference"))
  (bind _values (`BlueprintMapLibrary.Map_Values` (`self.NameToDeviceMap`)))
  (for _array_element _values
    (bind _returnvalue (`|SpawnActorFromClass` "/CesiumG2Visualization/G2VisualizationActors/NetBoxActors/BP_Netbox_Device.BP_Netbox_Device_C" (`KismetMathLibrary.MakeTransform` (0.0 0.0 0.0)) "Undefined" "OverrideRootScale" (`local.G2 Topology`) (`Device.IP` _array_element) (`Device.Info` _array_element) (`Device.MTU` _array_element) (`Device.Primary` _array_element) (`Device.ID` _array_element) (`Device.Url` _array_element) (`Device.Display` _array_element) (`Device.Name` _array_element) 0.0 0.0 (`local.G2 Topology`) null))
    (`self.K2_AttachToActor` _returnvalue self "None" "KeepRelative" "KeepRelative" "KeepRelative" true)
    ;[1 1 1] Copy Device Data
    (bind _output_get (set `/CesiumG2Visualization/G2VisualizationActors/NetBoxActors/BP_Netbox_Device.Site` (`BlueprintMapLibrary.Map_Find` (`local.Name to Site Map`) (`Site.Name` (`Device.Site` _array_element))) _returnvalue))
    (`KismetArrayLibrary.Array_Add` (`/CesiumG2Visualization/G2VisualizationActors/NetBoxActors/BP_Netbox_Site.Devices` _output_get) _returnvalue)
    (bind _location (`Device.Location` _array_element))
    (if (`KismetSystemLibrary.IsValid` _location)
      (bind _output_get_2 (set `/CesiumG2Visualization/G2VisualizationActors/NetBoxActors/BP_Netbox_Device.Location` (`BlueprintMapLibrary.Map_Find` (`local.Name to Location Map`) (`Location.Name` _location)) _returnvalue))
      (`KismetArrayLibrary.Array_Add` (`/CesiumG2Visualization/G2VisualizationActors/NetBoxActors/BP_Netbox_Location.Devices` _output_get_2) _returnvalue))))

(fn `Create Locations`
  (params (`Created Name To Site Map` :type "Map of String to /CesiumG2Visualization/G2VisualizationActors/NetBoxActors/BP_Netbox_Site Object Reference") (`G2 Topology` :type "/CesiumG2Visualization/BP_G2_Topology Object Reference"))
  (returns (`Created Name To Location Map` :type "Map of String to /CesiumG2Visualization/G2VisualizationActors/NetBoxActors/BP_Netbox_Location Object Reference"))
  (locals (`Name To Location Map` :type "Map of String to /CesiumG2Visualization/G2VisualizationActors/NetBoxActors/BP_Netbox_Location Object Reference"))
  (bind _name_to_location_map (`local.Name To Location Map`))
  (bind _values (`BlueprintMapLibrary.Map_Values` (`self.NameToLocationMap`)))
  (for _array_element _values
    (bind _returnvalue (`|SpawnActorFromClass` "/CesiumG2Visualization/G2VisualizationActors/NetBoxActors/BP_Netbox_Location.BP_Netbox_Location_C" (`KismetMathLibrary.MakeTransform` (0.0 0.0 0.0)) "Undefined" "OverrideRootScale" (`local.G2 Topology`) (`Location.Slug` _array_element) (`Location.LocationWorldLocationOffset` _array_element) (`Location.LocationWorldRotationOffset` _array_element) (`Location.ID` _array_element) (`Location.Url` _array_element) (`Location.Display` _array_element) (`Location.Name` _array_element) 0.0 0.0 (`local.G2 Topology`) null))
    (bind _output_get (set `/CesiumG2Visualization/G2VisualizationActors/NetBoxActors/BP_Netbox_Location.Site` (`BlueprintMapLibrary.Map_Find` (`local.Created Name To Site Map`) (`Site.Name` (`Location.Site` _array_element))) _returnvalue))
    (`KismetArrayLibrary.Array_Add` (`/CesiumG2Visualization/G2VisualizationActors/NetBoxActors/BP_Netbox_Site.Locations` _output_get) _returnvalue)
    (`self.K2_AttachToActor` _returnvalue _output_get "None" "KeepRelative" "KeepRelative" "KeepRelative" true)
    (`BlueprintMapLibrary.Map_Add` (`local.Name To Location Map`) (`/CesiumG2Visualization/G2VisualizationActors/NetBoxActors/BP_Netbox_Actor.Name` _returnvalue) _returnvalue))
  (for _array_element_2 _values
    (bind _parent (`Location.Parent` _array_element_2))
    (if (`KismetSystemLibrary.IsValid` _parent)
      (set `/CesiumG2Visualization/G2VisualizationActors/NetBoxActors/BP_Netbox_Location.Parent` (`BlueprintMapLibrary.Map_Find` _name_to_location_map (`Location.Name` _parent)) (`BlueprintMapLibrary.Map_Find` _name_to_location_map (`Location.Name` _array_element_2)))))
  (return (`local.Name To Location Map`)))

(fn `Create Regions`
  (params (`G2 Topology` :type "/CesiumG2Visualization/BP_G2_Topology Object Reference"))
  (returns (`Name to Region Map` :type "Map of String to /CesiumG2Visualization/G2VisualizationActors/NetBoxActors/BP_Netbox_Region Object Reference"))
  (locals (`Name to Region Map ` :type "Map of String to /CesiumG2Visualization/G2VisualizationActors/NetBoxActors/BP_Netbox_Region Object Reference"))
  (bind _name_to_region_map_ (`local.Name to Region Map `))
  (bind _values (`BlueprintMapLibrary.Map_Values` (`self.NameToRegionMap`)))
  (for _array_element _values
    (bind _returnvalue (`|SpawnActorFromClass` "/CesiumG2Visualization/G2VisualizationActors/NetBoxActors/BP_Netbox_Region.BP_Netbox_Region_C" (`KismetMathLibrary.MakeTransform` (0.0 0.0 0.0)) "Undefined" "OverrideRootScale" (`local.G2 Topology`) (`Region.Slug` _array_element) (`Region.Description` _array_element) (`Region.LogoUrl` _array_element) (`Region.ID` _array_element) (`Region.Url` _array_element) (`Region.Display` _array_element) (`Region.Name` _array_element) (`Region.Latitude` _array_element) (`Region.Longitude` _array_element) (`local.G2 Topology`) null))
    (`self.K2_AttachToActor` _returnvalue self "None" "KeepRelative" "KeepRelative" "KeepRelative" true)
    (`BlueprintMapLibrary.Map_Add` (`local.Name to Region Map `) (`/CesiumG2Visualization/G2VisualizationActors/NetBoxActors/BP_Netbox_Actor.Name` _returnvalue) _returnvalue))
  (for _array_element_2 _values
    (bind (_value _returnvalue_2) (`BlueprintMapLibrary.Map_Find` _name_to_region_map_ (`Region.ParentName` _array_element_2)))
    (if _returnvalue_2
      (set `/CesiumG2Visualization/G2VisualizationActors/NetBoxActors/BP_Netbox_Region.Parent` _value (`BlueprintMapLibrary.Map_Find` _name_to_region_map_ (`Region.Name` _array_element_2)))))
  (return (`local.Name to Region Map `)))

(fn `Create Replicated Actors`
  (params (`G2 Topology` :type "/CesiumG2Visualization/BP_G2_Topology Object Reference"))
  (returns (`Created Regions` :type "Array of /CesiumG2Visualization/G2VisualizationActors/NetBoxActors/BP_Netbox_Region Object Reference") (`Created Sites` :type "Array of /CesiumG2Visualization/G2VisualizationActors/NetBoxActors/BP_Netbox_Site Object Reference") (`Created Locations` :type "Array of /CesiumG2Visualization/G2VisualizationActors/NetBoxActors/BP_Netbox_Location Object Reference"))
  (bind _name_to_region_map (`self.Create Regions` `G2 Topology`))
  (bind _created_name_to_site_map (`self.Create Sites` _name_to_region_map `G2 Topology`))
  (bind _created_name_to_location_map (`self.Create Locations` _created_name_to_site_map `G2 Topology`))
  (bind _values (`BlueprintMapLibrary.Map_Values` _name_to_region_map))
  (bind _values_2 (`BlueprintMapLibrary.Map_Values` _created_name_to_site_map))
  (bind _values_3 (`BlueprintMapLibrary.Map_Values` _created_name_to_location_map))
  (return _values _values_2 _values_3))

(fn `Create Sites`
  (params (`Created Name to Region Map` :type "Map of String to /CesiumG2Visualization/G2VisualizationActors/NetBoxActors/BP_Netbox_Region Object Reference") (`G2 Topology` :type "/CesiumG2Visualization/BP_G2_Topology Object Reference"))
  (returns (`Created Name to Site Map` :type "Map of String to /CesiumG2Visualization/G2VisualizationActors/NetBoxActors/BP_Netbox_Site Object Reference"))
  (locals (`Name to Site Map` :type "Map of String to /CesiumG2Visualization/G2VisualizationActors/NetBoxActors/BP_Netbox_Site Object Reference"))
  (bind _values (`BlueprintMapLibrary.Map_Values` (`self.NameToSiteMap`)))
  (for _array_element _values
    (bind _returnvalue (`|SpawnActorFromClass` "/CesiumG2Visualization/G2VisualizationActors/NetBoxActors/BP_Netbox_Site.BP_Netbox_Site_C" (`KismetMathLibrary.MakeTransform` (0.0 0.0 0.0)) "Undefined" "OverrideRootScale" (`local.G2 Topology`) (`Site.Slug` _array_element) (`Site.ID` _array_element) (`Site.Url` _array_element) (`Site.Display` _array_element) (`Site.Name` _array_element) (`Site.Latitude` _array_element) (`Site.Longitude` _array_element) (`local.G2 Topology`) null))
    (`self.K2_AttachToActor` _returnvalue self "None" "KeepRelative" "KeepRelative" "KeepRelative" true)
    (`BlueprintMapLibrary.Map_Add` (`local.Name to Site Map`) (`/CesiumG2Visualization/G2VisualizationActors/NetBoxActors/BP_Netbox_Actor.Name` _returnvalue) _returnvalue)
    (bind (_value _returnvalue_2) (`BlueprintMapLibrary.Map_Find` (`local.Created Name to Region Map`) (`Site.RegionName` _array_element)))
    (if _returnvalue_2
      (bind _output_get (set `/CesiumG2Visualization/G2VisualizationActors/NetBoxActors/BP_Netbox_Site.Region` _value _returnvalue))
      (`KismetArrayLibrary.Array_Add` (`/CesiumG2Visualization/G2VisualizationActors/NetBoxActors/BP_Netbox_Region.Sites` _output_get) _returnvalue)))
  (return (`local.Name to Site Map`)))

(fn `Is Valid Lat Long`
  (params (Latitude :type "Float (double-precision)") (Longitude :type "Float (double-precision)"))
  (returns (ValidPoint :type Boolean))
  (locals (KansasLatitude :type "Float (double-precision)" :default 37.750999) (KansasLongitude :type "Float (double-precision)" :default -97.821999))
  (return (`KismetMathLibrary.BooleanNAND` (== Latitude (`local.KansasLatitude`)) (== Longitude (`local.KansasLongitude`)))))

(fn `Refresh`
  (set `self.Snapshot Load Started` true)
  (set `self.Snapshot Loaded` false)
  (bind _returnvalue (`|GenericCreateObject` "/Script/CesiumG2Visualization.G2Snapshot"))
  (set `self.Snapshot` _returnvalue)
  (`self.RequestBearerToken`))

(fn `Update Netbox Device`
  (params (Device :type "/CesiumG2Visualization/G2VisualizationActors/NetBoxActors/BP_Netbox_Device Object Reference"))
  (`self.RequestNetboxDevicePatch` null))

(fn `Update Netbox Location`
  (params (Location :type "/CesiumG2Visualization/G2VisualizationActors/NetBoxActors/BP_Netbox_Location Object Reference"))
  (`self.RequestNetboxLocationPatch` (`/CesiumG2Visualization/G2VisualizationActors/NetBoxActors/BP_Netbox_Location.ToStruct` Location)))

(fn `Update Netbox Rack`
  (params (Rack :type "/CesiumG2Visualization/G2VisualizationActors/NetBoxActors/BP_Netbox_Rack Object Reference"))
  (`self.RequestNetboxRackPatch` (`/CesiumG2Visualization/G2VisualizationActors/NetBoxActors/BP_Netbox_Rack.To Struct` Rack)))

(fn `Update Netbox Region`
  (params (Region :type "/CesiumG2Visualization/G2VisualizationActors/NetBoxActors/BP_Netbox_Region Object Reference"))
  (`self.RequestNetboxRegionPatch` (`/CesiumG2Visualization/G2VisualizationActors/NetBoxActors/BP_Netbox_Region.ToStruct` Region)))

(fn `Update Netbox Site`
  (params (Site :type "/CesiumG2Visualization/G2VisualizationActors/NetBoxActors/BP_Netbox_Site Object Reference"))
  (`self.RequestNetboxSitePatch` (`/CesiumG2Visualization/G2VisualizationActors/NetBoxActors/BP_Netbox_Site.ToStruct` Site)))

(fn `UserConstructionScript`)