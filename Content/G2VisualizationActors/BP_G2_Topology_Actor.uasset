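; Topology actor Blueprint for G2 visualization, apparently a base class, with helpers that range-check geographic coordinates.
; Latitude and longitude validators feed a combined check, and a class getter returns a fixed enum value.
; Color, static mesh scale setup, press and selection functions are empty stubs, and the construction script and events do nothing.
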(fn `Get G2 Topology Actor Class`
  (returns (NewParam :type "/CesiumG2Visualization/G2VisualizationActors/G2TopologyActorClass Enum"))
  (return "NewEnumerator1"))

(fn `On Pressed`)

(fn `On Selected`)

(fn `Set Color`)

(fn `Setup Static Mesh Component`
  (params (`New Scale` :type "Vector Structure")))

(fn `UserConstructionScript`)

(fn `Valid Latitude`
  (params (Latitude :type "Float (double-precision)"))
  (returns (Valid :type Boolean))
  (return (`KismetMathLibrary.InRange_FloatFloat` Latitude -90.0 90.0)))

(fn `Valid Latitude Longitude`
  (params (Latitude :type "Float (double-precision)") (Longitude :type "Float (double-precision)"))
  (returns (Valid :type Boolean))
  (return (and (`self.Valid Latitude` Latitude) (`self.Valid Longitude` Longitude))))

(fn `Valid Longitude`
  (params (Longitude :type "Float (double-precision)"))
  (returns (Valid :type Boolean))
  (return (`KismetMathLibrary.InRange_FloatFloat` Longitude -180.0 180.0)))