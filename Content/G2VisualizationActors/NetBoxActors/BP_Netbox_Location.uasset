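; Actor representing a NetBox Location in the G2 topology visualization, drawn as an orange cylinder with a dynamic material.
; UpdateData resolves Site and parent Location by name from the topology snapshot, re-attaches to the Site and applies the record's fields.
; ToStruct exports the record back, with relative position and rotation stored as custom-field strings that UpdateData parses.
; Press and selection events are forwarded to G2Topology.
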(fn `Change Site`
  (params (`New Site` :type "/CesiumG2Visualization/G2VisualizationActors/NetBoxActors/BP_Netbox_Site Object Reference"))
  (`KismetArrayLibrary.Array_RemoveItem` (`/CesiumG2Visualization/G2VisualizationActors/NetBoxActors/BP_Netbox_Site.Locations` (`self.Site`)) self)
  (bind _output_get (set `self.Site` `New Site`))
  (`self.K2_AttachToActor` _output_get "None" "KeepRelative" "KeepRelative" "KeepRelative")
  (`KismetArrayLibrary.Array_Add` (`/CesiumG2Visualization/G2VisualizationActors/NetBoxActors/BP_Netbox_Site.Locations` _output_get) self))

(fn `Get G2 Topology Actor Class`
  (returns (NewParam :type "/CesiumG2Visualization/G2VisualizationActors/G2TopologyActorClass Enum"))
  (return "NewEnumerator4"))

(fn `On Pressed`
  (`/CesiumG2Visualization/BP_G2_Topology.OnLocationPressed` (`self.G2 Topology`) self))

(fn `On Selected`
  (`/CesiumG2Visualization/BP_G2_Topology.OnLocationSelected` (`self.G2 Topology`) self))

(fn `Set Color`
  (`MaterialInstanceDynamic.SetVectorParameterValue` (`self.Dynamic Material`) "Color" (struct :`R` 1.0 :`G` 0.438973 :`B` 0.049112 :`A` 1.0)))

(fn `Setup Static Mesh Component`
  (params (`New Scale` :type "Vector Structure"))
  (bind _returnvalue (`|AddComponentByClass` "/CesiumG2Visualization/BP_Static_Mesh_Component.BP_Static_Mesh_Component_C"))
  (`SceneComponent.SetRelativeScale3D` _returnvalue `New Scale`)
  (`StaticMeshComponent.SetStaticMesh` _returnvalue "/Engine/BasicShapes/Cylinder.Cylinder")
  (set `self.Static Mesh Component` _returnvalue)
  (bind _returnvalue_2 (`PrimitiveComponent.CreateDynamicMaterialInstance` _returnvalue 0 "/CesiumG2Visualization/G2VisualizationActors/NetBoxActors/M_Device.M_Device" "None"))
  (set `self.Dynamic Material` _returnvalue_2))

(fn `ToStruct`
  (returns (Struct :type "LocationStruct Structure"))
  (locals (OutStruct :type "LocationStruct Structure"))
  (bind _parent (`self.Parent`))
  (bind _site (`self.Site`))
  (bind (_returnvalue_location _returnvalue_rotation) (`KismetMathLibrary.BreakTransform` (`SceneComponent.GetRelativeTransform` (`self.DefaultSceneRoot`))))
  (set `local.OutStruct` (make `LocationStruct` :`Id` (`self.Id`) :`Url` (`self.Url`) :`Display` (`self.Display`) :`Name` (`self.Name`) :`Slug` (`self.Slug`) :`Site` (make `LocationSite` -1) :`Parent` (make `LocationParent` -1) :`Custom_fields` (make `CustomLocationFields` (`KismetStringLibrary.Conv_VectorToString` _returnvalue_location) (`KismetStringLibrary.Conv_RotatorToString` _returnvalue_rotation))))
  (if (not (== (`self.Site`) null))
    (bind _structout (setmembers `LocationStruct` :`StructRef` (`local.OutStruct`) :`Site` (make `LocationSite` (`/CesiumG2Visualization/G2VisualizationActors/NetBoxActors/BP_Netbox_Actor.Id` _site) (`/CesiumG2Visualization/G2VisualizationActors/NetBoxActors/BP_Netbox_Actor.Url` _site) (`/CesiumG2Visualization/G2VisualizationActors/NetBoxActors/BP_Netbox_Actor.Display` _site) (`/CesiumG2Visualization/G2VisualizationActors/NetBoxActors/BP_Netbox_Actor.Name` _site) (`/CesiumG2Visualization/G2VisualizationActors/NetBoxActors/BP_Netbox_Site.Slug` _site))))
    (set `local.OutStruct` _structout))
  (if (not (== (`self.Parent`) null))
    (bind _structout_2 (setmembers `LocationStruct` :`StructRef` (`local.OutStruct`) :`Parent` (make `LocationParent` (`/CesiumG2Visualization/G2VisualizationActors/NetBoxActors/BP_Netbox_Actor.Id` _parent) (`/CesiumG2Visualization/G2VisualizationActors/NetBoxActors/BP_Netbox_Actor.Url` _parent) (`/CesiumG2Visualization/G2VisualizationActors/NetBoxActors/BP_Netbox_Actor.Display` _parent) (`/CesiumG2Visualization/G2VisualizationActors/NetBoxActors/BP_Netbox_Actor.Name` _parent) (`/Game/G2VisualizationActors/NetBoxActors/BP_Netbox_Location.Slug` _parent) 1)))
    (set `local.OutStruct` _structout_2))
  (return (`local.OutStruct`)))

(fn `Update Data`
  (params (`New Data` :type "LocationStruct Structure"))
  (bind (_id _url _display _name _slug _site _parent _tenant _tags _custom_fields) (break `LocationStruct` `New Data`))
  (bind (_id_2 _url_2 _display_2 _name_2 _slug_2 _site_2 _parent_2) (break `LocationStruct` `New Data`))
  (bind (_location_world_location_offset _location_world_rotation_offset) (break `CustomLocationFields` _custom_fields))
  (bind _snapshot (`/CesiumG2Visualization/BP_G2_Topology.Snapshot` (`self.G2 Topology`)))
  (`self.Change Site` (`BlueprintMapLibrary.Map_Find` (`/CesiumG2Visualization/BP_G2_Snapshot.Name to Site Map` _snapshot) (`.Name` (break `LocationSite` _site_2))))
  (set `self.Parent` (`BlueprintMapLibrary.Map_Find` (`/CesiumG2Visualization/BP_G2_Snapshot.Name to Location Map` _snapshot) (`.Name` (break `LocationParent` _parent_2))))
  (set `self.Id` _id)
  (set `self.Url` _url)
  (set `self.Display` _display)
  (set `self.Name` _name)
  (set `self.Slug` _slug)
  (`SceneComponent.K2_SetRelativeTransform` (`self.DefaultSceneRoot`) (`KismetMathLibrary.MakeTransform` (`KismetStringLibrary.Conv_StringToVector` _location_world_location_offset) (`KismetStringLibrary.Conv_StringToRotator` _location_world_rotation_offset)) false false))

(fn `UserConstructionScript`)