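; BP_Netbox_Site is a topology visualization actor for a NetBox site, holding its identity, coordinates, devices and parent region.
; It updates from incoming data via the topology snapshot's region lookup, converts itself to a site struct, and can switch regions.
; A runtime cylinder mesh with a green dynamic material represents it.
; Press, select and move events are forwarded to G2Topology, with moves using a server call.
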(fn `ChangeRegion`
  (params (`New Region Name` :type "/CesiumG2Visualization/G2VisualizationActors/NetBoxActors/BP_Netbox_Region Object Reference"))
  (`KismetArrayLibrary.Array_RemoveItem` (`/CesiumG2Visualization/G2VisualizationActors/NetBoxActors/BP_Netbox_Region.Sites` (`self.Region`)) self)
  (set `self.Region` `New Region Name`)
  (`KismetArrayLibrary.Array_Add` (`/CesiumG2Visualization/G2VisualizationActors/NetBoxActors/BP_Netbox_Region.Sites` `New Region Name`) self))

(fn `Get G2 Topology Actor Class`
  (returns (NewParam :type "/CesiumG2Visualization/G2VisualizationActors/G2TopologyActorClass Enum"))
  (return "NewEnumerator1"))

(fn `On Move`
  (params (`New Latitude` :type "Float (double-precision)") (`New Longitude` :type "Float (double-precision)"))
  (`/CesiumG2Visualization/BP_G2_Topology.On Move G2 Topology Actor SERVER` (`self.G2 Topology`) self `New Latitude` `New Longitude`))

(fn `On Pressed`
  (`/CesiumG2Visualization/BP_G2_Topology.OnSitePressed` (`self.G2 Topology`) self))

(fn `On Selected`
  (`/CesiumG2Visualization/BP_G2_Topology.OnSiteSelected` (`self.G2 Topology`) self))

(fn `Set Color`
  (`MaterialInstanceDynamic.SetVectorParameterValue` (`self.Dynamic Material`) "Color" (struct :`G` 0.44375 :`B` 0.089353 :`A` 1.0)))

(fn `Setup Static Mesh Component`
  (params (`New Scale` :type "Vector Structure"))
  (bind _returnvalue (`|AddComponentByClass` "/CesiumG2Visualization/BP_Static_Mesh_Component.BP_Static_Mesh_Component_C"))
  (`SceneComponent.SetRelativeScale3D` _returnvalue `New Scale`)
  (`StaticMeshComponent.SetStaticMesh` _returnvalue "/Engine/BasicShapes/Cylinder.Cylinder")
  (set `self.Static Mesh Component` _returnvalue)
  (bind _returnvalue_2 (`PrimitiveComponent.CreateDynamicMaterialInstance` _returnvalue 0 "/CesiumG2Visualization/G2VisualizationActors/NetBoxActors/M_Site.M_Site" "None"))
  (set `self.Dynamic Material` _returnvalue_2))

(fn `ToStruct`
  (returns (`Site Data` :type "SiteStruct Structure"))
  (bind _region (`self.Region`))
  (bind _sitestruct (make `SiteStruct` :`Id` (`self.Id`) :`Url` (`self.Url`) :`Display` (`self.Display`) :`Name` (`self.Name`) :`Slug` (`self.Slug`) :`Latitude` (`self.Latitude`) :`Longitude` (`self.Longitude`) :`Device_count` (`KismetArrayLibrary.Array_Length` (`self.Devices`))))
  (if (== (`self.Region`) null)
    (return _sitestruct)
    (else
      (bind _structout (setmembers `SiteStruct` :`StructRef` _sitestruct :`Region` (make `SiteRegion` (`KismetStringLibrary.Conv_IntToString` (`/CesiumG2Visualization/G2VisualizationActors/NetBoxActors/BP_Netbox_Actor.Id` _region)) (`/CesiumG2Visualization/G2VisualizationActors/NetBoxActors/BP_Netbox_Actor.Url` _region) (`/CesiumG2Visualization/G2VisualizationActors/NetBoxActors/BP_Netbox_Actor.Display` _region) (`/CesiumG2Visualization/G2VisualizationActors/NetBoxActors/BP_Netbox_Actor.Name` _region) (`/CesiumG2Visualization/G2VisualizationActors/NetBoxActors/BP_Netbox_Region.Slug` _region) 1)))
      (return _structout))))

(fn `Update Data`
  (params (`New Data` :type "SiteStruct Structure"))
  (bind (_id _url _display _name _slug _status _region _group _tenant _facility _time_zone _description _physical_address _shipping_address _latitude _longitude) (break `SiteStruct` `New Data`))
  (set `self.Region` (`BlueprintMapLibrary.Map_Find` (`/CesiumG2Visualization/BP_G2_Snapshot.Name to Region Map` (`/CesiumG2Visualization/BP_G2_Topology.Snapshot` (`self.G2 Topology`))) (`.Name` (break `SiteRegion` (`.Region` (break `SiteStruct` `New Data`))))))
  (set `self.Id` _id)
  (set `self.Url` _url)
  (set `self.Display` _display)
  (set `self.Name` _name)
  (set `self.Slug` _slug)
  (set `self.Latitude` _latitude)
  (set `self.Longitude` _longitude))

(fn `UserConstructionScript`)