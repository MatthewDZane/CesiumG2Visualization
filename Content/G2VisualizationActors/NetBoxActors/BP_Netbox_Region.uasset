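; Actor representing a NetBox region in the G2 topology visualization, holding its metadata, coordinates, parent and sites.
; Builds a ring mesh with a dynamic material colored by whether it has sites, and spawns an attached 3D info display.
; Converts data to and from region structs, resolving parents by name, and downloads its logo to refresh the display.
; Forwards press, select and server move events to the topology actor.
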(event `self.ReceiveBeginPlay`)

(event `On Download Logo`
  (bind _logo_url (`self.Logo Url`))
  (if (not (`KismetStringLibrary.IsEmpty` _logo_url))
    (bind _texture (`AsyncTaskDownloadImage.DownloadImage` _logo_url)
      (:`OnSuccess`
        (set `self.Logo` _texture)
        (`KismetSystemLibrary.PrintString` (`KismetStringLibrary.Concat_StrStr` "Image Downloaded Successfully: " _logo_url))
        (bind _asregion_display (cast `/CesiumG2Visualization/Widgets/RegionWidgets/RegionDisplay` (`WidgetComponent.GetUserWidgetObject` (`/CesiumG2Visualization/G2VisualizationActors/NetBoxActors/BP_3D_Region_Display.Region Display` (`self.3D Display`)))))
        (message `/CesiumG2Visualization/Widgets/DataDisplay.Update Info` _asregion_display))
      (:`OnFail`
        (`KismetSystemLibrary.PrintString` (`KismetStringLibrary.Concat_StrStr` "Image Url was invalid:" _logo_url))))))

(fn `ChangeParent`
  (params (`New Parent Name` :type String))
  (bind _asbp_g2_topology (cast `/CesiumG2Visualization/BP_G2_Topology` (`self.GetAttachParentActor`)))
  (set `/Game/G2VisualizationActors/NetBoxActors/BP_Netbox_Region.Parent` null (`BlueprintMapLibrary.Map_Find` (`/CesiumG2Visualization/BP_G2_Snapshot.Name to Region Map` (`/CesiumG2Visualization/BP_G2_Topology.Snapshot` _asbp_g2_topology)) `New Parent Name`)))

(fn `Get G2 Topology Actor Class`
  (returns (NewParam :type "/CesiumG2Visualization/G2VisualizationActors/G2TopologyActorClass Enum"))
  (return "NewEnumerator0"))

(fn `On Move`
  (params (`New Latitude` :type "Float (double-precision)") (`New Longitude` :type "Float (double-precision)"))
  (`/CesiumG2Visualization/BP_G2_Topology.On Move G2 Topology Actor SERVER` (`self.G2 Topology`) self `New Latitude` `New Longitude`))

(fn `On Pressed`
  (`/CesiumG2Visualization/BP_G2_Topology.OnRegionPressed` (`self.G2 Topology`) self))

(fn `On Selected`
  (`/CesiumG2Visualization/BP_G2_Topology.OnRegionSelected` (`self.G2 Topology`) self))

(fn `Set Color`
  (bind _dynamic_material (`self.Dynamic Material`))
  (if (> (`KismetArrayLibrary.Array_Length` (`self.Sites`)) 0)
    (`MaterialInstanceDynamic.SetVectorParameterValue` _dynamic_material "Color" (struct :`R` 1.0 :`G` 0.312223 :`A` 1.0))
    (else
      (`MaterialInstanceDynamic.SetVectorParameterValue` _dynamic_material "Color" (struct :`R` 0.234375 :`G` 0.234375 :`B` 0.234375 :`A` 1.0)))))

(fn `Setup 3D Display`
  (params (`Small Setting` :type Boolean))
  (bind _returnvalue (`|SpawnActorFromClass` "/CesiumG2Visualization/G2VisualizationActors/NetBoxActors/BP_3D_Region_Display.BP_3D_Region_Display_C" (`KismetMathLibrary.MakeTransform` (0.0 0.0 0.0)) "Undefined" "OverrideRootScale" null `Small Setting` null))
  (bind _output_get (set `self.3D Display` _returnvalue))
  (`self.K2_AttachToActor` _output_get self "None" "KeepRelative" "KeepRelative" "KeepRelative" true)
  (bind _asregion_display (cast `/CesiumG2Visualization/Widgets/RegionWidgets/RegionDisplay` (`WidgetComponent.GetUserWidgetObject` (`/CesiumG2Visualization/G2VisualizationActors/NetBoxActors/BP_3D_Region_Display.Region Display` (`self.3D Display`)))))
  (message `/CesiumG2Visualization/Widgets/DataDisplay.Set Info` _asregion_display self))

(fn `Setup Static Mesh Component`
  (params (`New Scale` :type "Vector Structure"))
  (bind _returnvalue (`|AddComponentByClass` "/CesiumG2Visualization/BP_Static_Mesh_Component.BP_Static_Mesh_Component_C"))
  (`SceneComponent.SetRelativeScale3D` _returnvalue `New Scale`)
  (`StaticMeshComponent.SetStaticMesh` _returnvalue "/CesiumG2Visualization/G2VisualizationActors/NetBoxActors/RingMesh.RingMesh")
  (set `self.Static Mesh Component` _returnvalue)
  (bind _returnvalue_2 (`PrimitiveComponent.CreateDynamicMaterialInstance` _returnvalue 0 "/CesiumG2Visualization/G2VisualizationActors/NetBoxActors/M_Region.M_Region" "None"))
  (set `self.Dynamic Material` _returnvalue_2))

(fn `ToStruct`
  (returns (`Region Data` :type "RegionStruct Structure"))
  (bind _regionstruct (make `RegionStruct` :`Id` (`self.Id`) :`Url` (`self.Url`) :`Display` (`self.Display`) :`Name` (`self.Name`) :`Slug` (`self.Slug`) :`Description` (`self.Description`) :`Custom_fields` (make `CustomRegionFields` (`self.Logo Url`) (`KismetStringLibrary.Conv_DoubleToString` (`self.Latitude`)) (`KismetStringLibrary.Conv_DoubleToString` (`self.Longitude`))) :`Site_count` (`KismetArrayLibrary.Array_Length` (`self.Sites`))))
  (if (== (`self.Parent`) null)
    (return _regionstruct)
    (else
      (bind _structout (setmembers `RegionStruct` :`StructRef` _regionstruct :`Parent` (make `RegionParent` (`KismetStringLibrary.Conv_IntToString` (`self.Id`)) (`self.Url`) (`self.Display`) (`self.Name`) (`/Game/G2VisualizationActors/NetBoxActors/BP_Netbox_Region.Slug` (`self.Parent`)) 1)))
      (return _structout))))

(fn `Update Data`
  (params (`New Data` :type "RegionStruct Structure"))
  (bind (_id _url _display _name _slug _parent _description _tags _custom_fields) (break `RegionStruct` `New Data`))
  (bind (_logo _region_latitude _region_longitude) (break `CustomRegionFields` _custom_fields))
  (set `self.Parent` (`BlueprintMapLibrary.Map_Find` (`/CesiumG2Visualization/BP_G2_Snapshot.Name to Region Map` (`/CesiumG2Visualization/BP_G2_Topology.Snapshot` (`self.G2 Topology`))) (`.Name` (break `RegionParent` (`.Parent` (break `RegionStruct` `New Data`))))))
  (set `self.Id` _id)
  (set `self.Url` _url)
  (set `self.Display` _display)
  (set `self.Name` _name)
  (set `self.Slug` _slug)
  (set `self.Description` _description)
  (set `self.Logo Url` _logo)
  (set `self.Latitude` (`KismetStringLibrary.Conv_StringToDouble` _region_latitude))
  (set `self.Longitude` (`KismetStringLibrary.Conv_StringToDouble` _region_longitude)))

(fn `UserConstructionScript`)