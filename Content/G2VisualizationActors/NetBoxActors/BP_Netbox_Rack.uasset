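; BP_Netbox_Rack is an actor representing a NetBox rack in the G2 topology visualization.
; UpdateData copies identity fields from incoming data, resolves its Site and Location by name through the snapshot maps, and parses world location and rotation offsets from custom-field strings.
; ToStruct rebuilds a rack struct from that state, adding site and location references when valid.
; Selection reports the rack to NetBoxVisualization through OnLocationSelected.
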(fn `Get G2 Topology Actor Class`
  (returns (NewParam :type "/CesiumNetBoxVisualization/G2VisualizationActors/G2TopologyActorClass Enum"))
  (return "NewEnumerator5"))

(fn `On Selected`
  (`/CesiumNetBoxVisualization/BP_G2_Topology.OnLocationSelected` (`self.NetBox Visualization`) self))

(fn `To Struct`
  (returns (Struct :type "RackStruct Structure"))
  (locals (`Out Struct` :type "RackStruct Structure"))
  (bind _location (`self.Location`))
  (bind _site (`self.Site`))
  (set `local.Out Struct` (make `RackStruct` :`Id` (`self.Id`) :`Url` (`self.Url`) :`Display` (`self.Display`) :`Name` (`self.Name`) :`Custom_fields` (make `CustomRackFields` 0.0 0.0 (`KismetStringLibrary.Conv_VectorToString` (`self.World Location Offset`)) (`KismetStringLibrary.Conv_RotatorToString` (`self.World Rotator Offset`)))))
  (if (`KismetSystemLibrary.IsValid` _site)
    (setmembers `RackStruct` :`StructRef` (`local.Out Struct`) :`Site` (make `RackSite` (`/CesiumNetBoxVisualization/G2VisualizationActors/NetBoxActors/BP_Netbox_Actor.Id` _site) (`/CesiumNetBoxVisualization/G2VisualizationActors/NetBoxActors/BP_Netbox_Actor.Url` _site) (`/CesiumNetBoxVisualization/G2VisualizationActors/NetBoxActors/BP_Netbox_Actor.Display` _site) (`/CesiumNetBoxVisualization/G2VisualizationActors/NetBoxActors/BP_Netbox_Actor.Name` _site) (`/CesiumNetBoxVisualization/G2VisualizationActors/NetBoxActors/BP_Netbox_Site.Slug` _site))))
  (if (`KismetSystemLibrary.IsValid` _location)
    (setmembers `RackStruct` :`StructRef` (`local.Out Struct`) :`Location` (make `RackLocation` (`/CesiumNetBoxVisualization/G2VisualizationActors/NetBoxActors/BP_Netbox_Actor.Id` _location) (`/CesiumNetBoxVisualization/G2VisualizationActors/NetBoxActors/BP_Netbox_Actor.Url` _location) (`/CesiumNetBoxVisualization/G2VisualizationActors/NetBoxActors/BP_Netbox_Actor.Display` _location) (`/CesiumNetBoxVisualization/G2VisualizationActors/NetBoxActors/BP_Netbox_Actor.Name` _location) (`/CesiumNetBoxVisualization/G2VisualizationActors/NetBoxActors/BP_Netbox_Location.Slug` _location))))
  (return (`local.Out Struct`)))

(fn `Update Data`
  (params (`New Data` :type "RackStruct Structure"))
  (locals (NewLocalVar_0 :type "RackLocation Structure"))
  (bind (_id _url _display _name _facility_id _site _location) (break `RackStruct` `New Data`))
  (bind (_id_2 _url_2 _display_2 _name_2 _facility_id_2 _site_2 _location_2 _tenant _status _role _serial _asset_tag _type _width _u_height _desc_units _outer_width _outer_depth _outer_unit _comments _tags _custom_fields) (break `RackStruct` `New Data`))
  (bind (_rack_latitude _rack_longitude _rack_world_location_offset _rack_world_rotation_offset) (break `CustomRackFields` _custom_fields))
  (bind _snapshot (`/CesiumNetBoxVisualization/BP_G2_Topology.Snapshot` (`self.NetBox Visualization`)))
  (set `self.Site` (`BlueprintMapLibrary.Map_Find` (`/CesiumNetBoxVisualization/BP_G2_Snapshot.Name to Site Map` _snapshot) (`.Name` (break `RackSite` _site))))
  (set `self.Location` (`BlueprintMapLibrary.Map_Find` (`/CesiumNetBoxVisualization/BP_G2_Snapshot.Name to Location Map` _snapshot) (`.Name` (break `RackLocation` _location))))
  (set `self.Id` _id_2)
  (set `self.Url` _url_2)
  (set `self.Display` _display_2)
  (set `self.Name` _name_2)
  (set `self.World Location Offset` (`KismetStringLibrary.Conv_StringToVector` _rack_world_location_offset))
  (set `self.World Rotator Offset` (`KismetStringLibrary.Conv_StringToRotator` _rack_world_rotation_offset)))

(fn `UserConstructionScript`)