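; Actor representing a NetBox device in the G2 topology visualization, drawn as a cube with a yellow-tintable dynamic material.
; UpdateData copies device fields and resolves Site, Location and Rack through the topology snapshot's name maps, while ToStruct packs them back into a struct.
; Latitude and longitude come from the Site, and ChangeSite moves the device between sites and notifies the topology.
; Press and selection events forward to the topology actor.
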(fn `Change Site`
  (params (NewSiteName :type String))
  (bind _asbp_g2_topology (cast `/CesiumG2Visualization/BP_G2_Topology` (`self.GetAttachParentActor`)))
  (`KismetArrayLibrary.Array_RemoveItem` (`/CesiumG2Visualization/G2VisualizationActors/NetBoxActors/BP_Netbox_Site.Devices` (`self.Site`)) self)
  (bind _value (`BlueprintMapLibrary.Map_Find` (`/CesiumG2Visualization/BP_G2_Snapshot.Name to Site Map` (`/CesiumG2Visualization/BP_G2_Topology.Snapshot` _asbp_g2_topology)) NewSiteName))
  (set `self.Site` _value)
  (`KismetArrayLibrary.Array_Add` (`/CesiumG2Visualization/G2VisualizationActors/NetBoxActors/BP_Netbox_Site.Devices` _value) self)
  (`/CesiumG2Visualization/BP_G2_Topology.On Handle Actor Release` _asbp_g2_topology _value))

(fn `Get G2 Topology Actor Class`
  (returns (NewParam :type "/CesiumG2Visualization/G2VisualizationActors/G2TopologyActorClass Enum"))
  (return "NewEnumerator6"))

(fn `Get Latitude`
  (returns (Latitude :type "Float (double-precision)"))
  (return (`/CesiumG2Visualization/G2VisualizationActors/NetBoxActors/BP_Netbox_Actor.Latitude` (`self.Site`))))

(fn `Get Longitude`
  (returns (Longitude :type "Float (double-precision)"))
  (return (`/CesiumG2Visualization/G2VisualizationActors/NetBoxActors/BP_Netbox_Actor.Longitude` (`self.Site`))))

(fn `On Pressed`
  (`/CesiumG2Visualization/BP_G2_Topology.OnDevicePressed` (`self.G2 Topology`) self))

(fn `On Selected`
  (`/CesiumG2Visualization/BP_G2_Topology.OnDeviceSelected` (`self.G2 Topology`) self))

(fn `Set Color`
  (`MaterialInstanceDynamic.SetVectorParameterValue` (`self.Dynamic Material`) "Color" (struct :`R` 1.0 :`G` 0.917677 :`B` 0.020335 :`A` 1.0)))

(fn `Setup Static Mesh Component`
  (params (`New Scale` :type "Vector Structure"))
  (bind _returnvalue (`|AddComponentByClass` "/CesiumG2Visualization/BP_Static_Mesh_Component.BP_Static_Mesh_Component_C"))
  (`SceneComponent.SetRelativeScale3D` _returnvalue `New Scale`)
  (`StaticMeshComponent.SetStaticMesh` _returnvalue "/Engine/BasicShapes/Cube.Cube")
  (set `self.Static Mesh Component` _returnvalue)
  (bind _returnvalue_2 (`PrimitiveComponent.CreateDynamicMaterialInstance` _returnvalue 0 "/CesiumG2Visualization/G2VisualizationActors/NetBoxActors/M_Device.M_Device" "None"))
  (set `self.Dynamic Material` _returnvalue_2))

(fn `To Struct`
  (returns (Struct :type "DeviceStruct Structure"))
  (locals (`Out Struct` :type "DeviceStruct Structure"))
  (bind _location (`self.Location`))
  (bind _rack (`self.Rack`))
  (bind _site (`self.Site`))
  (set `local.Out Struct` (make `DeviceStruct` :`Id` (`self.Id`) :`Url` (`self.Url`) :`Display` (`self.Display`) :`Name` (`self.Name`) :`Primary_ip` (make `PrimaryIp` 0 "" "" "" (`self.IP`)) :`Custom_fields` (make `CustomDeviceFields` (`self.Info`) (`self.MTU`) (`self.Primary`))))
  (if (`KismetSystemLibrary.IsValid` _site)
    (setmembers `DeviceStruct` :`StructRef` (`local.Out Struct`) :`Site` (make `DeviceSite` (`/CesiumG2Visualization/G2VisualizationActors/NetBoxActors/BP_Netbox_Actor.Id` _site) (`/CesiumG2Visualization/G2VisualizationActors/NetBoxActors/BP_Netbox_Actor.Url` _site) (`/CesiumG2Visualization/G2VisualizationActors/NetBoxActors/BP_Netbox_Actor.Display` _site) (`/CesiumG2Visualization/G2VisualizationActors/NetBoxActors/BP_Netbox_Actor.Name` _site) (`/CesiumG2Visualization/G2VisualizationActors/NetBoxActors/BP_Netbox_Site.Slug` _site))))
  (if (`KismetSystemLibrary.IsValid` _location)
    (setmembers `DeviceStruct` :`StructRef` (`local.Out Struct`) :`Location` (make `DeviceLocation` (`/CesiumG2Visualization/G2VisualizationActors/NetBoxActors/BP_Netbox_Actor.Id` _location) (`/CesiumG2Visualization/G2VisualizationActors/NetBoxActors/BP_Netbox_Actor.Url` _location) (`/CesiumG2Visualization/G2VisualizationActors/NetBoxActors/BP_Netbox_Actor.Display` _location) (`/CesiumG2Visualization/G2VisualizationActors/NetBoxActors/BP_Netbox_Actor.Name` _location) (`/CesiumG2Visualization/G2VisualizationActors/NetBoxActors/BP_Netbox_Location.Slug` _location))))
  (if (`KismetSystemLibrary.IsValid` _rack)
    (setmembers `DeviceStruct` :`StructRef` (`local.Out Struct`) :`Rack` (make `DeviceRack` (`/CesiumG2Visualization/G2VisualizationActors/NetBoxActors/BP_Netbox_Actor.Id` _rack) (`/CesiumG2Visualization/G2VisualizationActors/NetBoxActors/BP_Netbox_Actor.Url` _rack) (`/CesiumG2Visualization/G2VisualizationActors/NetBoxActors/BP_Netbox_Actor.Display` _rack) (`/CesiumG2Visualization/G2VisualizationActors/NetBoxActors/BP_Netbox_Actor.Name` _rack))))
  (return (`local.Out Struct`)))

(fn `Update Data`
  (params (`New Data` :type "DeviceStruct Structure"))
  (bind (_id _url _display _name _device_type _device_role _tenant _platform _serial _asset_tag _site _location _rack) (break `DeviceStruct` `New Data`))
  (bind (_id_2 _url_2 _display_2 _name_2 _device_type_2 _device_role_2 _tenant_2 _platform_2 _serial_2 _asset_tag_2 _site_2 _location_2 _rack_2 _position _face _parent_device _status _airflow _primary_ip _primary_ip4 _primary_ip6 _cluster _virtual_chassis _vc_position _vc_priority _comments _local_context_data _tags _custom_fields) (break `DeviceStruct` `New Data`))
  (bind (_info _mtu _primary) (break `CustomDeviceFields` _custom_fields))
  (bind _snapshot (`/CesiumG2Visualization/BP_G2_Topology.Snapshot` (`self.G2 Topology`)))
  (set `self.Site` (`BlueprintMapLibrary.Map_Find` (`/CesiumG2Visualization/BP_G2_Snapshot.Name to Site Map` _snapshot) (`.Name` (break `DeviceSite` _site))))
  (set `self.Location` (`BlueprintMapLibrary.Map_Find` (`/CesiumG2Visualization/BP_G2_Snapshot.Name to Location Map` _snapshot) (`.Name` (break `DeviceLocation` _location))))
  (set `self.Rack` (`BlueprintMapLibrary.Map_Find` (`/CesiumG2Visualization/BP_G2_Snapshot.Name to Rack Map` _snapshot) (`.Name` (break `DeviceRack` _rack))))
  (set `self.Id` _id_2)
  (set `self.Url` _url_2)
  (set `self.Display` _display_2)
  (set `self.Name` _name_2)
  (set `self.IP` (`.Address` (break `PrimaryIp` _primary_ip)))
  (set `self.Info` _info)
  (set `self.MTU` _mtu)
  (set `self.Primary` _primary))

(fn `UserConstructionScript`)