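; Cesium globe version of the G2 topology visualization, placing Netbox regions, sites, locations, devices and nodes on Earth, joined by spline-mesh links.
; Setup events attach globe anchors, orient actors to the surface and collect untethered nodes and links.
; Pawn altitude drives Global, Region, Site and Location view modes, which switch visibility, scale, lerp speed and simulation.
; Releasing a site or device lerps its children toward it.
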(event `self.ReceiveBeginPlay`
  (`parent.ReceiveBeginPlay`)
  (bind _returnvalue (`CesiumGeoreference.GetDefaultGeoreference`))
  (bind _returnvalue_2 (`CesiumGeoreference.TransformEcefToUnreal` _returnvalue (0.0 0.0 0.0)))
  (set `self.Planet Radius` (`KismetMathLibrary.Vector_Distance` (`CesiumGeoreference.TransformLongitudeLatitudeHeightToUnreal` _returnvalue (117.0 43.0 100.0)) _returnvalue_2))
  (set `self.Center of Earth` _returnvalue_2)
  (set `self.Link Force Constant` 0.2)
  (set `self.Planet Radius Center Force Offset` 10000.0)
  (set `self.Center Force Constant ` 0.25)
  (set `self.Center Repulsion Force Constant` 200000000.0)
  (set `self.Min Earth Distance` 1.0)
  (set `self.MTU Force Constant` 1000.0)
  (set `self.Tangent Friction Force Constant` 0.25)
  (set `self.Center Friction Force Constant` 0.9)
  (set `self.LERP Speed` 125000000.0)
  (set `self.Overlapping Distance Threshold` 10000.0))

(event `self.ReceiveTick`
  (params (DeltaSeconds :type "Float (single-precision)"))
  (`parent.ReceiveTick` DeltaSeconds)
  (`self.Check View Mode Change`))

(event `/CesiumG2Visualization/BP_G2_Topology_Interface.Setup Regions`
  (bind _values (`BlueprintMapLibrary.Map_Values` (`/CesiumG2Visualization/BP_G2_Snapshot.Name to Region Map` (`self.Snapshot`))))
  (for _array_element _values
    (`/Engine/EditorBlueprintResources/ActorMacros.Switch Has Authority`
      (:`Authority`
        (bind _returnvalue (`|AddComponentByClass` _array_element "/Script/CesiumRuntime.CesiumGlobeAnchorComponent"))
        (bind _output_get (set `/CesiumG2Visualization/G2VisualizationActors/BP_G2_Topology_Actor.Cesium Globe` _returnvalue _array_element))
        (`CesiumGlobeAnchorComponent.MoveToLongitudeLatitudeHeight` _output_get (`KismetMathLibrary.MakeVector` (`/CesiumG2Visualization/G2VisualizationActors/NetBoxActors/BP_Netbox_Actor.Get Longitude` _array_element) (`/CesiumG2Visualization/G2VisualizationActors/NetBoxActors/BP_Netbox_Actor.Get Latitude` _array_element) 1000.0))
        (`self.K2_SetActorRelativeRotation` _array_element (`self.GetRotationRelativeToSurface` (`self.GetRelativeLocation` _array_element)) false false))
      (:`Remote`
        _))
    (`/CesiumG2Visualization/G2VisualizationActors/BP_G2_Topology_Actor.Setup Static Mesh Component` _array_element (50000.0 50000.0 10000.0))
    (`/CesiumG2Visualization/G2VisualizationActors/BP_G2_Topology_Actor.Set Color` _array_element)
    (`/CesiumG2Visualization/G2VisualizationActors/NetBoxActors/BP_Netbox_Region.Setup 3D Display` _array_element false)
    (`/CesiumG2Visualization/G2VisualizationActors/NetBoxActors/BP_Netbox_Region.On Download Logo` _array_element)))

(event `/CesiumG2Visualization/BP_G2_Topology_Interface.Setup Sites`
  (bind _values (`BlueprintMapLibrary.Map_Values` (`/CesiumG2Visualization/BP_G2_Snapshot.Name to Site Map` (`self.Snapshot`))))
  (for _array_element _values
    (`/Engine/EditorBlueprintResources/ActorMacros.Switch Has Authority`
      (:`Authority`
        (bind _returnvalue (`|AddComponentByClass` _array_element "/Script/CesiumRuntime.CesiumGlobeAnchorComponent"))
        (bind _output_get (set `/CesiumG2Visualization/G2VisualizationActors/BP_G2_Topology_Actor.Cesium Globe` _returnvalue _array_element))
        (`CesiumGlobeAnchorComponent.MoveToLongitudeLatitudeHeight` _output_get (`KismetMathLibrary.MakeVector` (`/CesiumG2Visualization/G2VisualizationActors/NetBoxActors/BP_Netbox_Actor.Get Longitude` _array_element) (`/CesiumG2Visualization/G2VisualizationActors/NetBoxActors/BP_Netbox_Actor.Get Latitude` _array_element) 200.0))
        (bind _region (`/CesiumG2Visualization/G2VisualizationActors/NetBoxActors/BP_Netbox_Site.Region` _array_element))
        (if (and (not (`self.Is Valid Location` (`/CesiumG2Visualization/G2VisualizationActors/NetBoxActors/BP_Netbox_Actor.Latitude` _array_element) (`/CesiumG2Visualization/G2VisualizationActors/NetBoxActors/BP_Netbox_Actor.Longitude` _array_element))) (`KismetSystemLibrary.IsValid` _region))
          (`self.On Move G2 Topology Actor SERVER` _array_element (`/CesiumG2Visualization/G2VisualizationActors/NetBoxActors/BP_Netbox_Actor.Latitude` _region) (`/CesiumG2Visualization/G2VisualizationActors/NetBoxActors/BP_Netbox_Actor.Latitude` _region)))
        (`self.K2_SetActorRelativeRotation` _array_element (`self.GetRotationRelativeToSurface` (`self.GetRelativeLocation` _array_element)) false false))
      (:`Remote`
        _))
    (`/CesiumG2Visualization/G2VisualizationActors/BP_G2_Topology_Actor.Setup Static Mesh Component` _array_element (1.0 1.0 1.0))
    (`/CesiumG2Visualization/G2VisualizationActors/BP_G2_Topology_Actor.Set Color` _array_element)))

(event `/CesiumG2Visualization/BP_G2_Topology_Interface.Setup Locations`
  (bind _values (`BlueprintMapLibrary.Map_Values` (`/CesiumG2Visualization/BP_G2_Snapshot.Name to Location Map` (`self.Snapshot`))))
  (for _array_element _values
    (`self.K2_SetActorRelativeTransform` _array_element (`KismetMathLibrary.MakeTransform` (`/CesiumG2Visualization/G2VisualizationActors/NetBoxActors/BP_Netbox_Location.World Location Offset` _array_element) (`/CesiumG2Visualization/G2VisualizationActors/NetBoxActors/BP_Netbox_Location.World Rotator Offset` _array_element)) false false)
    (`/CesiumG2Visualization/G2VisualizationActors/BP_G2_Topology_Actor.Setup Static Mesh Component` _array_element (100.0 100.0 10.0))
    (`/CesiumG2Visualization/G2VisualizationActors/BP_G2_Topology_Actor.Set Color` _array_element)
    (`SceneComponent.K2_SetRelativeRotation` (`/CesiumG2Visualization/G2VisualizationActors/BP_G2_Topology_Actor.Static Mesh Component` _array_element) (`self.GetRotationRelativeToSurface` (`self.GetRelativeLocation` _array_element)) false false)
    (`/Engine/EditorBlueprintResources/ActorMacros.Switch Has Authority`
      (:`Authority`
        (bind _returnvalue (`|AddComponentByClass` _array_element "/Script/CesiumRuntime.CesiumGlobeAnchorComponent"))
        (bind _output_get (set `/CesiumG2Visualization/G2VisualizationActors/BP_G2_Topology_Actor.Cesium Globe` _returnvalue _array_element))
        (bind (_returnvalue_x _returnvalue_y) (`KismetMathLibrary.BreakVector` (`CesiumGlobeAnchorComponent.GetLongitudeLatitudeHeight` _output_get)))
        (set `/CesiumG2Visualization/G2VisualizationActors/NetBoxActors/BP_Netbox_Actor.Latitude` _returnvalue_y _array_element)
        (set `/CesiumG2Visualization/G2VisualizationActors/NetBoxActors/BP_Netbox_Actor.Longitude` _returnvalue_x _array_element)))))

(event `/CesiumG2Visualization/BP_G2_Topology_Interface.Setup Devices`
  (bind _values (`BlueprintMapLibrary.Map_Values` (`/CesiumG2Visualization/BP_G2_Snapshot.Name to Device Map` (`self.Snapshot`))))
  (for _array_element _values
    (bind _returnvalue (`|AddComponentByClass` _array_element "/Script/CesiumRuntime.CesiumGlobeAnchorComponent"))
    (bind _output_get (set `/CesiumG2Visualization/G2VisualizationActors/BP_G2_Topology_Actor.Cesium Globe` _returnvalue _array_element))
    (`CesiumGlobeAnchorComponent.MoveToLongitudeLatitudeHeight` _output_get (`KismetMathLibrary.MakeVector` (`/CesiumG2Visualization/G2VisualizationActors/NetBoxActors/BP_Netbox_Actor.Get Longitude` _array_element) (`/CesiumG2Visualization/G2VisualizationActors/NetBoxActors/BP_Netbox_Actor.Get Latitude` _array_element) 200.0))
    (`self.K2_SetActorRelativeRotation` _array_element (`self.GetRotationRelativeToSurface` (`self.GetRelativeLocation` _array_element)) false false)
    (`/CesiumG2Visualization/G2VisualizationActors/BP_G2_Topology_Actor.Setup Static Mesh Component` _array_element (1.0 1.0 1.0))
    (`/CesiumG2Visualization/G2VisualizationActors/BP_G2_Topology_Actor.Set Color` _array_element)
    (bind _name (`/CesiumG2Visualization/G2VisualizationActors/NetBoxActors/BP_Netbox_Actor.Name` _array_element))
    (`BlueprintMapLibrary.Map_Add` (`/CesiumG2Visualization/BP_G2_Snapshot.Name to Device Map` (`self.Snapshot`)) _name _array_element)
    (`ComboBoxString.AddOption` (`/CesiumG2Visualization/Widgets/NodeWidgets/NodeDataDisplay.DeviceComboBox` (`self.Node Data Display`)) _name)))

(event `/CesiumG2Visualization/BP_G2_Topology_Interface.Setup Nodes`
  (bind _values (`BlueprintMapLibrary.Map_Values` (`/CesiumG2Visualization/BP_G2_Snapshot.ID to Node Map` (`self.Snapshot`))))
  (for _array_element _values
    ;[1 1 1] If node found but location invalid, add to the list of Untethered Nodes
    (if (`/CesiumG2Visualization/G2VisualizationActors/BP_G2_Node.Untethered` _array_element)
      (`self.Create Untethered Node` _array_element))
    (bind _returnvalue (`|AddComponentByClass` _array_element "/Script/CesiumRuntime.CesiumGlobeAnchorComponent"))
    (bind _output_get (set `/CesiumG2Visualization/G2VisualizationActors/BP_G2_Topology_Actor.Cesium Globe` _returnvalue _array_element))
    (`CesiumGlobeAnchorComponent.MoveToLongitudeLatitudeHeight` _output_get (`KismetMathLibrary.MakeVector` (`/CesiumG2Visualization/G2VisualizationActors/BP_G2_Node.Get Longitude` _array_element) (`/CesiumG2Visualization/G2VisualizationActors/BP_G2_Node.Get Latitude` _array_element) 250000.0))
    (`self.K2_SetActorRelativeRotation` _array_element (`self.GetRotationRelativeToSurface` (`self.GetRelativeLocation` _array_element)) false false)
    (`/CesiumG2Visualization/G2VisualizationActors/BP_G2_Node.Setup Static Mesh Component` _array_element (20000.0 20000.0 20000.0)) ; Any modifications to the mesh must be made after here
    (`/CesiumG2Visualization/G2VisualizationActors/BP_G2_Node.Set Color` _array_element)))

(event `/CesiumG2Visualization/BP_G2_Topology_Interface.Setup Links`
  ;[1 1 1] Setup Links
  (for _array_element (`/CesiumG2Visualization/BP_G2_Snapshot.Links` (`self.Snapshot`))
    (set `/CesiumG2Visualization/G2VisualizationActors/BP_G2_Link.Min Curve Angel` 1.0 _array_element)
    (if (or (`/CesiumG2Visualization/G2VisualizationActors/BP_G2_Node.Untethered` (`/CesiumG2Visualization/G2VisualizationActors/BP_G2_Link.Source` _array_element)) (`/CesiumG2Visualization/G2VisualizationActors/BP_G2_Node.Untethered` (`/CesiumG2Visualization/G2VisualizationActors/BP_G2_Link.Target` _array_element)))
      (`KismetArrayLibrary.Array_Add` (`self.Untethered Links`) _array_element))
    ;;[1 1 1] Create Spline Component
    (bind _returnvalue (`AddComponent|NODE_AddSplineComponent-0` :`self` _array_element))
    (bind _output_get (set `/CesiumG2Visualization/G2VisualizationActors/BP_G2_Link.Spline Component` _returnvalue _array_element))
    (for _ (range (+ (- (`self.Spline Length`) 2) 1))
      (`SplineComponent.AddSplinePoint` _output_get (`KismetMathLibrary.Vector_Zero`) "Local" true))
    (for _ (range (`self.Spline Length`))
      ;;[1 1 1] Add Mesh to point i to i+1
      (bind _returnvalue_2 (`AddComponent|NODE_AddSplineMeshComponent-0` :`self` _array_element))
      (`KismetArrayLibrary.Array_Add` (`/CesiumG2Visualization/G2VisualizationActors/BP_G2_Link.Spline Mesh Component I` _array_element) _returnvalue_2)
      (`SplineMeshComponent.SetStartScale` _returnvalue_2 (10000.0 10000.0) true)
      (`SplineMeshComponent.SetEndScale` _returnvalue_2 (10000.0 10000.0) true)
      (`SceneComponent.K2_AttachToComponent` _returnvalue_2 (`/CesiumG2Visualization/G2VisualizationActors/BP_G2_Link.DefaultSceneRoot` _array_element) "None" "KeepRelative" "KeepRelative" "KeepRelative" false)))
  (for _array_element_2 (`/CesiumG2Visualization/BP_G2_Snapshot.Links` (`self.Snapshot`))
    (`/CesiumG2Visualization/G2VisualizationActors/BP_G2_Link.Set Color ` _array_element_2 10000.0)
    (`/CesiumG2Visualization/G2VisualizationActors/BP_G2_Link.UpdateSpline` _array_element_2 (`self.Spline Length`) (`self.Planet Radius`) (`self.Curve Height`) (`self.Center of Earth`))))

(event `self.On Handle Actor Release`
  (params (`Released Actor` :type "Actor Object Reference"))
  (bind _asbp_netbox_site (cast `/CesiumG2Visualization/G2VisualizationActors/NetBoxActors/BP_Netbox_Site` `Released Actor`)
    (:`then`
      (if (`/CesiumG2Visualization/G2VisualizationActors/NetBoxActors/BP_Netbox_Actor.Location Set` _asbp_netbox_site)
        (for _array_element (`/CesiumG2Visualization/G2VisualizationActors/NetBoxActors/BP_Netbox_Site.Devices` _asbp_netbox_site)
          (`self.Add LERPing Actor` _array_element (`KismetMathLibrary.InverseTransformLocation` (`self.GetTransform`) (`self.K2_GetActorLocation` _asbp_netbox_site))))))
    (:`CastFailed`
      (bind _asbp_netbox_device (cast `/CesiumG2Visualization/G2VisualizationActors/NetBoxActors/BP_Netbox_Device` `Released Actor`))
      (if (`/CesiumG2Visualization/G2VisualizationActors/NetBoxActors/BP_Netbox_Actor.Location Set` (`/CesiumG2Visualization/G2VisualizationActors/NetBoxActors/BP_Netbox_Device.Site` _asbp_netbox_device))
        (for _array_element_2 (`/CesiumG2Visualization/G2VisualizationActors/NetBoxActors/BP_Netbox_Device.Nodes` _asbp_netbox_device)
          (`self.Add LERPing Actor` _array_element_2 (`KismetMathLibrary.InverseTransformLocation` (`self.GetTransform`) (`self.K2_GetActorLocation` _asbp_netbox_device))))))))

(event `self.On Move G2 Topology Actor SERVER`
  (params (`G2 Topology Actor` :type "/CesiumG2Visualization/G2VisualizationActors/BP_G2_Topology_Actor Object Reference") (Latitude :type "Float (double-precision)") (Longitude :type "Float (double-precision)"))
  (bind (_returnvalue_x _returnvalue_y _returnvalue_z) (`KismetMathLibrary.BreakVector` (`CesiumGlobeAnchorComponent.GetLongitudeLatitudeHeight` (`/CesiumG2Visualization/G2VisualizationActors/BP_G2_Topology_Actor.Cesium Globe` `G2 Topology Actor`))))
  (bind _returnvalue (`CesiumGeoreference.GetDefaultGeoreference`))
  (`self.Add LERPing Actor` `G2 Topology Actor` (`CesiumGeoreference.TransformLongitudeLatitudeHeightToUnreal` _returnvalue (`KismetMathLibrary.MakeVector` Longitude Latitude _returnvalue_z))))

(fn `Add LERPing Actor`
  (params (`Actor To LERP` :type "Actor Object Reference (by ref)") (`Target Local Location` :type "Vector Structure (by ref)"))
  (`parent.Add LERPing Actor` `Actor To LERP` `Target Local Location`)
  (return))

(fn `Change View Mode`
  (params (`New Mode` :type "/CesiumG2Visualization/G2TopologyViewMode Enum" :default "NewEnumerator0"))
  (set `self.Current View Mode` `New Mode`)
  (`self.Update Actor Visibilities`)
  (`self.Update Actor Scales`)
  (`self.Update LERP Speed`)
  (switch `/CesiumG2Visualization/G2TopologyViewMode` (`self.Current View Mode`)
    (:`NewEnumerator0`
      (`KismetSystemLibrary.PrintString` "Global View"))
    (:`NewEnumerator1`
      (`KismetSystemLibrary.PrintString` "Region View"))
    (:`NewEnumerator2`
      (`KismetSystemLibrary.PrintString` "Site View"))
    (:`NewEnumerator3`
      (`KismetSystemLibrary.PrintString` "Location View"))))

(fn `Check View Mode Change`
  (locals (`Current Altitude` :type "Float (double-precision)"))
  (bind _asbp_g2_visualization_cesium_pawn (cast `/CesiumG2Visualization/BP_G2_Visualization_Cesium_Pawn` (`GameplayStatics.GetPlayerPawn` 0)))
  (bind (_returnvalue_x _returnvalue_y _returnvalue_z) (`KismetMathLibrary.BreakVector` (`CesiumGlobeAnchorComponent.GetLongitudeLatitudeHeight` (`GlobeAwareDefaultPawn.GlobeAnchor` _asbp_g2_visualization_cesium_pawn))))
  (set `local.Current Altitude` _returnvalue_z)
  (switch `/CesiumG2Visualization/G2TopologyViewMode` (`self.Current View Mode`)
    (:`NewEnumerator0`
      (if (< (`local.Current Altitude`) (`self.Global To Region Transition Altitude`))
        (`self.Change View Mode` "NewEnumerator1")))
    (:`NewEnumerator1`
      (if (> (`local.Current Altitude`) (`self.Region to Global Transition Altitude`))
        (`self.Change View Mode` "NewEnumerator0")
        (elif (< (`local.Current Altitude`) (`self.Region To Site Transition Altitude`))
          (`self.Change View Mode` "NewEnumerator2"))))
    (:`NewEnumerator2`
      (`self.Update On Ground Netbox Actors`)
      (if (> (`local.Current Altitude`) (`self.Site To Region Transition Altitude`))
        (`self.Change View Mode` "NewEnumerator1")
        (elif (< (`local.Current Altitude`) (`self.Site to Location Transition Altitude`))
          (`self.Change View Mode` "NewEnumerator3"))))
    (:`NewEnumerator3`
      (if (> (`local.Current Altitude`) (`self.Location to Site Transition Altitude`))
        (`self.Change View Mode` "NewEnumerator2")))))

(fn `Get Transform from Lat Long`
  (params (Latitude :type "Float (double-precision)") (Longitude :type "Float (double-precision)"))
  (returns (ReturnValue :type "Transform Structure"))
  (bind _returnvalue (`CesiumGeoreference.GetDefaultGeoreference`))
  (bind _returnvalue_2 (`CesiumGeoreference.TransformLongitudeLatitudeHeightToUnreal` _returnvalue (`KismetMathLibrary.MakeVector` Longitude Latitude 10000.0)))
  (return (`KismetMathLibrary.MakeTransform` _returnvalue_2 (`self.GetRotationRelativeToSurface` _returnvalue_2))))

(fn `GetOverlappingSites`
  (params (Site :type "/CesiumG2Visualization/G2VisualizationActors/NetBoxActors/BP_Netbox_Site Object Reference"))
  (returns (OverlappingSites :type "Array of /CesiumG2Visualization/G2VisualizationActors/NetBoxActors/BP_Netbox_Site Object Reference"))
  (locals (`Found Overlapping Sites` :type "Array of /CesiumG2Visualization/G2VisualizationActors/NetBoxActors/BP_Netbox_Site Object Reference"))
  (bind _values (`BlueprintMapLibrary.Map_Values` (`/CesiumG2Visualization/BP_G2_Snapshot.Name to Site Map` (`self.Snapshot`))))
  (for _array_element _values
    (if (< (`self.GetDistanceTo` _array_element Site) 6250000.0)
      (`KismetArrayLibrary.Array_Add` (`local.Found Overlapping Sites`) _array_element)))
  (return (`local.Found Overlapping Sites`)))

(fn `GoIntoLocation`
  (params (Location :type "/CesiumG2Visualization/G2VisualizationActors/NetBoxActors/BP_Netbox_Location Object Reference"))
  (for _ (`/CesiumG2Visualization/G2VisualizationActors/NetBoxActors/BP_Netbox_Location.Racks` Location)
    _))

(fn `Restore Site Location`
  (params (Site :type "/CesiumG2Visualization/G2VisualizationActors/NetBoxActors/BP_Netbox_Site Object Reference"))
  (bind _returnvalue (`CesiumGeoreference.GetDefaultGeoreference`))
  (`self.Add LERPing Actor` Site (`CesiumGeoreference.TransformLongitudeLatitudeHeightToUnreal` _returnvalue (`KismetMathLibrary.MakeVector` (`/CesiumG2Visualization/G2VisualizationActors/NetBoxActors/BP_Netbox_Actor.Get Longitude` Site) (`/CesiumG2Visualization/G2VisualizationActors/NetBoxActors/BP_Netbox_Actor.Get Latitude` Site) 100.0))))

(fn `Set Device Scales`
  (params (NewRelativeScale :type "Vector Structure"))
  (bind _values (`BlueprintMapLibrary.Map_Values` (`/CesiumG2Visualization/BP_G2_Snapshot.Name to Device Map` (`self.Snapshot`))))
  (for _array_element _values
    (`SceneComponent.SetRelativeScale3D` (`/CesiumG2Visualization/G2VisualizationActors/BP_G2_Topology_Actor.Static Mesh Component` _array_element) NewRelativeScale)))

(fn `Set Devices To Hidden`
  (params (Hidden :type Boolean))
  (bind _values (`BlueprintMapLibrary.Map_Values` (`/CesiumG2Visualization/BP_G2_Snapshot.Name to Device Map` (`self.Snapshot`))))
  (for _array_element _values
    (`self.SetActorHiddenInGame` _array_element Hidden)
    (`self.SetActorEnableCollision` _array_element (not Hidden))))

(fn `Set Links to Hidden`
  (params (Hidden :type Boolean))
  (for _array_element (`/CesiumG2Visualization/BP_G2_Snapshot.Links` (`self.Snapshot`))
    (`self.SetActorHiddenInGame` _array_element Hidden)
    (`self.SetActorEnableCollision` _array_element (not Hidden))))

(fn `Set Locations To Hidden`
  (params (Hidden :type Boolean))
  (bind _values (`BlueprintMapLibrary.Map_Values` (`/CesiumG2Visualization/BP_G2_Snapshot.Name to Location Map` (`self.Snapshot`))))
  (for _array_element _values
    (`self.SetActorHiddenInGame` _array_element Hidden)
    (`self.SetActorEnableCollision` _array_element (not Hidden))))

(fn `Set Netbox Actors Hidden`
  (params (Hidden :type Boolean))
  (`self.Set Regions to Hidden` Hidden)
  (`self.Set Sites to Hidden` Hidden)
  (`self.Set Locations To Hidden` Hidden)
  (`self.Set Devices To Hidden` Hidden)
  (`self.Set Nodes To Hidden` Hidden)
  (`self.Set Links to Hidden` Hidden))

(fn `Set Nodes To Hidden`
  (params (Hidden :type Boolean))
  (bind _values (`BlueprintMapLibrary.Map_Values` (`/CesiumG2Visualization/BP_G2_Snapshot.ID to Node Map` (`self.Snapshot`))))
  (for _array_element _values
    (`self.SetActorHiddenInGame` _array_element Hidden)
    (`self.SetActorEnableCollision` _array_element (not Hidden))))

(fn `Set Regions to Hidden`
  (params (Hidden :type Boolean))
  (bind _returnvalue (not Hidden))
  (bind _values (`BlueprintMapLibrary.Map_Values` (`/CesiumG2Visualization/BP_G2_Snapshot.Name to Region Map` (`self.Snapshot`))))
  (for _array_element _values
    (`self.SetActorHiddenInGame` _array_element Hidden)
    (`self.SetActorHiddenInGame` (`/CesiumG2Visualization/G2VisualizationActors/NetBoxActors/BP_Netbox_Region.3D Display` _array_element) Hidden)
    (`self.SetActorEnableCollision` _array_element _returnvalue)
    (`self.SetActorEnableCollision` (`/CesiumG2Visualization/G2VisualizationActors/NetBoxActors/BP_Netbox_Region.3D Display` _array_element) _returnvalue)))

(fn `Set Site Scales`
  (params (NewRelativeScale :type "Vector Structure"))
  (bind _values (`BlueprintMapLibrary.Map_Values` (`/CesiumG2Visualization/BP_G2_Snapshot.Name to Site Map` (`self.Snapshot`))))
  (for _array_element _values
    (`SceneComponent.SetRelativeScale3D` (`/CesiumG2Visualization/G2VisualizationActors/BP_G2_Topology_Actor.Static Mesh Component` _array_element) NewRelativeScale)))

(fn `Set Sites to Hidden`
  (params (Hidden :type Boolean))
  (bind _values (`BlueprintMapLibrary.Map_Values` (`/CesiumG2Visualization/BP_G2_Snapshot.Name to Site Map` (`self.Snapshot`))))
  (for _array_element _values
    (`self.SetActorHiddenInGame` _array_element Hidden)
    (`self.SetActorEnableCollision` _array_element (not Hidden))))

(fn `Setup Region Data Display`
  (`parent.Setup Region Data Display`)
  (set `/CesiumG2Visualization/Widgets/RegionWidgets/RegionDataDisplay.Go Into Visible` true (`self.Region Data Display`)))

(fn `Setup Site Data Display`
  (`parent.Setup Site Data Display`)
  (set `/CesiumG2Visualization/Widgets/SiteWidgets/SiteDataDisplay.Go Into Visible` true (`self.Site Data Display`)))

(fn `Setup Visualization`
  (`parent.Setup Visualization`)
  (`self.Change View Mode` "NewEnumerator0"))

(fn `Update Actor Scales`
  (switch `/CesiumG2Visualization/G2TopologyViewMode` (`self.Current View Mode`)
    (:`NewEnumerator0`
      (`self.Set Site Scales` (`self.Global View Site Scale`))
      (`self.Set Device Scales` (`self.Global View Device Scale`)))
    (:`NewEnumerator1`
      (`self.Set Site Scales` (`self.Region View Site Scale`))
      (`self.Set Device Scales` (`self.Region View Device Scale`)))
    (:`NewEnumerator2`
      (`self.Set Device Scales` (`self.Site View Device Scale`)))))

(fn `Update Actor Visibilities`
  (switch `/CesiumG2Visualization/G2TopologyViewMode` (`self.Current View Mode`)
    (:`NewEnumerator0`
      (set `self.SimulationRunning` true)
      (`self.Set Netbox Actors Hidden` false)
      (`self.Set Locations To Hidden` true))
    (:`NewEnumerator1`
      (set `self.SimulationRunning` false)
      (`self.Set Regions to Hidden` true)
      (`self.Set Sites to Hidden` false)
      (`self.Set Locations To Hidden` true)
      (`self.Set Devices To Hidden` false)
      (`self.Set Nodes To Hidden` true)
      (`self.Set Links to Hidden` true))
    (:`NewEnumerator2`
      (set `self.SimulationRunning` false)
      (`self.Set Regions to Hidden` true)
      (`self.Set Sites to Hidden` true)
      (`self.Set Locations To Hidden` false)
      (`self.Set Devices To Hidden` false)
      (`self.Set Nodes To Hidden` true)
      (`self.Set Links to Hidden` true))
    (:`NewEnumerator3`
      (set `self.SimulationRunning` false)
      (`self.Set Regions to Hidden` true)
      (`self.Set Sites to Hidden` true)
      (`self.Set Locations To Hidden` false)
      (`self.Set Devices To Hidden` false)
      (`self.Set Nodes To Hidden` true)
      (`self.Set Links to Hidden` true))))

(fn `Update LERP Speed`
  (switch `/CesiumG2Visualization/G2TopologyViewMode` (`self.Current View Mode`)
    (:`NewEnumerator0`
      (set `self.LERP Speed` 125000000.0))
    (:`NewEnumerator1`
      (set `self.LERP Speed` 125000000.0))
    (:`NewEnumerator2`
      (set `self.LERP Speed` 0.0))
    (:`NewEnumerator3`
      (set `self.LERP Speed` 0.0))))

(fn `Update On Ground Netbox Actors`
  (switch `/CesiumG2Visualization/G2TopologyViewMode` (`self.Current View Mode`)))

(fn `UserConstructionScript`
  (`parent.UserConstructionScript`)
  (`ActorComponent.K2_DestroyComponent` (`self.Outward`))
  (`ActorComponent.K2_DestroyComponent` (`self.Inward`)))