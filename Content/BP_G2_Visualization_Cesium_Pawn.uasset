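; Cesium globe pawn for the G2 visualization, which flies between geographic locations with back and forward history and lets the user click, select and drag Netbox topology actors.
; A mouse trace dispatches clicks by actor class, resolving overlaps through the currently selected actor.
; While grabbing, Tick intersects the cursor ray with an Earth-centered sphere via the quadratic formula, preserving actor height.
; SERVER and MULTICAST events relay moves, saves and display updates.
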(event `self.ReceiveBeginPlay`
  (add `self.OnFlightInterrupt` (delegate `OnFlightInterrupt_Event`))
  (add `self.OnFlightComplete` (delegate `OnFlightComplete_Event`))
  (`parent.ReceiveBeginPlay`)
  (`self.Setup Restore Location Widget`)
  (`GameplayStatics.GetActorOfClass` "/Script/Engine.PlayerStart")
  (set `PlayerController.bShowMouseCursor` true (`GameplayStatics.GetPlayerController` 0))
  (bind _asbp_g2_visualization_player_controller (cast `/CesiumNetBoxVisualization/BP_G2_Visualization_PlayerController` (`GameplayStatics.GetPlayerController` 0))
    (:`then`
      (set `/CesiumNetBoxVisualization/BP_G2_Visualization_PlayerController.IsPossessDone` true _asbp_g2_visualization_player_controller))
    (:`CastFailed`
      _))
  (bind _asbp_g2_visualization_cesium_pawn (cast `/Game/BP_G2_Visualization_Cesium_Pawn` (`GameplayStatics.GetPlayerPawn` 0)))
  (`self.FlyToLocationLongitudeLatitudeHeight` _asbp_g2_visualization_cesium_pawn (-98.949091 38.490952 5000000.0) -89.99 -89.99 false)
  (`PlayerController.SetMouseCursorWidget` (`GameplayStatics.GetPlayerController` 0) "CardinalCross" null))

(event `OnFlightInterrupt_Event`
  (set `self.Flying` false :!label _label))

(event `OnFlightComplete_Event`
  (goto _label))

(event `Fly to Previous Location`
  (bind _currentlocationindex (`self.CurrentLocationIndex`))
  (if (not (`self.Flying`))
    (set `self.Flying` true)
    (if (> _currentlocationindex 0)
      (bind _result (`/Engine/EditorBlueprintResources/StandardMacros.DecrementInt` _currentlocationindex)
        (:`  `
          (`self.FlyToLocationLongitudeLatitudeHeight` (`|GetArrayItem` (`self.LastLocations`) _result) -89.999901 -89.999901 true))))))

(event `Fly to Forward Location`
  (bind _currentlocationindex (`self.CurrentLocationIndex`))
  (if (and (> (- (`KismetArrayLibrary.Array_Length` (`self.LastLocations`)) 1) _currentlocationindex) (not (`self.Flying`)))
    (set `self.Flying` true)
    (bind _result (`/Engine/EditorBlueprintResources/StandardMacros.IncrementInt` _currentlocationindex)
      (:`  `
        (`self.FlyToLocationLongitudeLatitudeHeight` (`|GetArrayItem` (`self.LastLocations`) _result) -89.999901 -89.999901 true)))))

(event `/CesiumNetBoxVisualization/BP_G2_Topology_Pawn_Interface.Move G2 Topology Actor`
  (params (`G2 Topology Actor` :type "/CesiumNetBoxVisualization/G2VisualizationActors/BP_G2_Topology_Actor Object Reference") (`New Relative Transformation` :type "Transform Structure"))
  ;[1 1 1] Netbox Interface
  (`self.Move G2 Topology Actor SERVER` `G2 Topology Actor` `New Relative Transformation`))

(event `Move G2 Topology Actor SERVER`
  (params (`G2 Topology Actor` :type "/CesiumNetBoxVisualization/G2VisualizationActors/BP_G2_Topology_Actor Object Reference") (`New Relative Transformation` :type "Transform Structure (by ref)"))
  ;[1 1 1] Netbox Interface
  (`self.K2_SetActorTransform` `G2 Topology Actor` `New Relative Transformation` false false)
  (`/CesiumNetBoxVisualization/BP_G2_Topology_Pawn_Interface.Update G2 Topology Actor Data Display` `G2 Topology Actor`))

(event `Fly to New Location Longitude Latitude Height`
  (params (`Longitude Latitude Height Destination` :type "Vector Structure"))
  (bind _lastlocations (`self.LastLocations`))
  (if (not (`self.Flying`))
    (set `self.Flying` true)
    (if (> (`KismetArrayLibrary.Array_Length` _lastlocations) 9)
      (`KismetArrayLibrary.Array_Remove` _lastlocations)
      (`/Engine/EditorBlueprintResources/StandardMacros.DecrementInt` (`self.CurrentLocationIndex`)
        (:`  `
          _)))
    (if (> (`KismetArrayLibrary.Array_Length` _lastlocations) 9)
      (`KismetArrayLibrary.Array_Remove` _lastlocations)
      (`/Engine/EditorBlueprintResources/StandardMacros.DecrementInt` (`self.CurrentLocationIndex`)
        (:`  `
          _)))
    (`KismetArrayLibrary.Array_Add` _lastlocations (`CesiumGlobeAnchorComponent.GetLongitudeLatitudeHeight` (`self.GlobeAnchor`)))
    (`KismetArrayLibrary.Array_Add` _lastlocations `Longitude Latitude Height Destination`)
    (bind _output_get (set `self.CurrentLocationIndex` (+ 2 (`self.CurrentLocationIndex`))))
    (`self.FlyToLocationLongitudeLatitudeHeight` `Longitude Latitude Height Destination` -89.999901 -89.999901 true)
    (for _ (range 1 (+ (- (`KismetArrayLibrary.Array_Length` (`self.LastLocations`)) _output_get 1) 1))
      (`KismetArrayLibrary.Array_Remove` (`self.LastLocations`) (+ _output_get 1)))))

(event `Update G2 Topology Actor Data Display SERVER`
  (params (`G2 Topology Actor` :type "/CesiumNetBoxVisualization/G2VisualizationActors/BP_G2_Topology_Actor Object Reference"))
  (bind (_returnvalue_x _returnvalue_y) (`KismetMathLibrary.BreakVector` (`CesiumGlobeAnchorComponent.GetLongitudeLatitudeHeight` (`/CesiumNetBoxVisualization/G2VisualizationActors/BP_G2_Topology_Actor.Cesium Globe` `G2 Topology Actor`))))
  ;[1 1 1] Netbox Interface
  (`self.Update G2 Topology Actor Data Display MULTICAST` `G2 Topology Actor` _returnvalue_y _returnvalue_x))

(event `/CesiumNetBoxVisualization/BP_G2_Topology_Pawn_Interface.Update G2 Topology Actor Data Display`
  (params (`G2 Topology Actor` :type "/CesiumNetBoxVisualization/G2VisualizationActors/BP_G2_Topology_Actor Object Reference"))
  ;[1 1 1] Netbox Interface
  (`self.Update G2 Topology Actor Data Display SERVER` `G2 Topology Actor`))

(event `Update G2 Topology Actor Data Display Latitude Longitude SERVER`
  (params (`G2 Topology Actor` :type "/CesiumNetBoxVisualization/G2VisualizationActors/BP_G2_Topology_Actor Object Reference") (`New Latitude` :type "Float (double-precision)") (`New Longitude` :type "Float (double-precision)"))
  ;[1 1 1] Netbox Interface
  (`self.Update G2 Topology Actor Data Display MULTICAST` `G2 Topology Actor` `New Latitude` `New Longitude`))

(event `/CesiumNetBoxVisualization/BP_G2_Topology_Pawn_Interface.Update G2 Topology Actor Data Display Latitude Longitude`
  (params (`G2 Topology Actor` :type "/CesiumNetBoxVisualization/G2VisualizationActors/BP_G2_Topology_Actor Object Reference") (Latitude :type "Float (double-precision)") (Longitude :type "Float (double-precision)"))
  ;[1 1 1] Netbox Interface
  (`self.Update G2 Topology Actor Data Display Latitude Longitude SERVER` `G2 Topology Actor` Latitude Longitude))

(event `Update G2 Topology Actor Data Display MULTICAST`
  (params (`G2 Topology Actor` :type "/CesiumNetBoxVisualization/G2VisualizationActors/BP_G2_Topology_Actor Object Reference") (Latitude :type "Float (double-precision)") (Longitude :type "Float (double-precision)"))
  ;[1 1 1] Netbox Interface
  (switch `/CesiumNetBoxVisualization/G2VisualizationActors/G2TopologyActorClass` (`/CesiumNetBoxVisualization/G2VisualizationActors/BP_G2_Topology_Actor.Get G2 Topology Actor Class` `G2 Topology Actor`)
    (:`NewEnumerator0`
      (bind _asbp_netbox_region (cast `/CesiumNetBoxVisualization/G2VisualizationActors/NetBoxActors/BP_Netbox_Region` `G2 Topology Actor`))
      (`self.Update Region Data Display` _asbp_netbox_region Latitude Longitude))
    (:`NewEnumerator1`
      (bind _asbp_netbox_site (cast `/CesiumNetBoxVisualization/G2VisualizationActors/NetBoxActors/BP_Netbox_Site` `G2 Topology Actor`))
      (`self.Update Site Data Display` _asbp_netbox_site Latitude Longitude))
    (:`NewEnumerator7`
      (bind _asbp_g2_node (cast `/CesiumNetBoxVisualization/G2VisualizationActors/BP_G2_Node` `G2 Topology Actor`))
      (`self.Update Node Data Display` _asbp_g2_node Latitude Longitude))))

(event `/CesiumNetBoxVisualization/BP_G2_Topology_Pawn_Interface.Move G2 Topology Actor to Latitude Longitude`
  (params (`G2 Topology Actor` :type "/CesiumNetBoxVisualization/G2VisualizationActors/BP_G2_Topology_Actor Object Reference") (Latitude :type "Float (double-precision)") (Longitude :type "Float (double-precision)"))
  ;[1 1 1] Netbox Interface
  (`self.Move G2 Topology Actor To Latitude Longitude SERVER` `G2 Topology Actor` Latitude Longitude))

(event `Move G2 Topology Actor To Latitude Longitude SERVER`
  (params (`G2 Topology Actor` :type "/CesiumNetBoxVisualization/G2VisualizationActors/BP_G2_Topology_Actor Object Reference") (Latitude :type "Float (double-precision)") (Longitude :type "Float (double-precision)"))
  ;[1 1 1] Netbox Interface
  (`/CesiumNetBoxVisualization/BP_G2_Topology.On Move G2 Topology Actor` (`/CesiumNetBoxVisualization/G2VisualizationActors/BP_G2_Topology_Actor.NetBox Visualization` `G2 Topology Actor`) `G2 Topology Actor` Latitude Longitude))

(event `Key|LeftMouseButton`
  (params (Key :type "Key Structure"))
  (bind _grabbed_netbox_actor (`self.Grabbed Netbox Actor`))
  (bind (_worldlocation _worlddirection) (`PlayerController.DeprojectMousePositionToWorld` (`GameplayStatics.GetPlayerController` 0)))
  (:`Pressed`
    (bind (_outhit _returnvalue) (`KismetSystemLibrary.LineTraceSingleForObjects` :`Start` _worldlocation :`End` (+ _worldlocation (* _worlddirection 99999999999.0)) :`ObjectTypes` (`|MakeArray` "ObjectTypeQuery1" "ObjectTypeQuery2" :!type "EObjectTypeQuery Enum") :`DrawDebugType` "ForDuration"))
    (if _returnvalue
      (`self.Handle Actor Clicked` (`.HitActor` (`GameplayStatics.BreakHitResult` _outhit)) (`.Distance` (`GameplayStatics.BreakHitResult` _outhit)) (`.Location` (`GameplayStatics.BreakHitResult` _outhit)))
      (else
        (set `self.GrabMode` false))))
  (:`Released`
    (if (`KismetSystemLibrary.IsValid` _grabbed_netbox_actor)
      (`/CesiumNetBoxVisualization/BP_G2_Topology_Pawn_Interface.Handle G2 Topology Actor Release` _grabbed_netbox_actor))
    (set `self.Grabbed Netbox Actor` null)
    (set `self.GrabMode` false)))

(event `/CesiumNetBoxVisualization/BP_G2_Topology_Pawn_Interface.Handle G2 Topology Actor Release`
  (params (`G2 Topology Actor` :type "/CesiumNetBoxVisualization/G2VisualizationActors/BP_G2_Topology_Actor Object Reference"))
  ;[1 1 1] Netbox Interface
  (`self.Handle G2 Topology Actor Release SERVER` `G2 Topology Actor`))

(event `Handle G2 Topology Actor Release SERVER`
  (params (`Released G2 Topology Actor` :type "/CesiumNetBoxVisualization/G2VisualizationActors/BP_G2_Topology_Actor Object Reference"))
  ;[1 1 1] Netbox Interface
  (`/CesiumNetBoxVisualization/BP_G2_Topology.On Handle Actor Release` (`/CesiumNetBoxVisualization/G2VisualizationActors/BP_G2_Topology_Actor.NetBox Visualization` `Released G2 Topology Actor`) `Released G2 Topology Actor`)
  (`self.Handle Actor Release MULTICAST` `Released G2 Topology Actor`))

(event `Handle Actor Release MULTICAST`
  (params (`Released G2 Topology Actor` :type "/CesiumNetBoxVisualization/G2VisualizationActors/BP_G2_Topology_Actor Object Reference"))
  ;[1 1 1] Netbox Interface
)

(event `On Save Region SERVER`
  (params (Region :type "/CesiumNetBoxVisualization/G2VisualizationActors/NetBoxActors/BP_Netbox_Region Object Reference") (`New Region Data` :type "RegionStruct Structure"))
  ;[1 1 1] Netbox Interface
  (`/CesiumNetBoxVisualization/BP_G2_Topology.On Save Region` (`/CesiumNetBoxVisualization/G2VisualizationActors/BP_G2_Topology_Actor.NetBox Visualization` Region) Region `New Region Data`))

(event `/CesiumNetBoxVisualization/BP_G2_Topology_Pawn_Interface.On Save Region`
  (params (Region :type "/CesiumNetBoxVisualization/G2VisualizationActors/NetBoxActors/BP_Netbox_Region Object Reference") (`New Region Data` :type "RegionStruct Structure"))
  ;[1 1 1] Netbox Interface
  (`self.On Save Region SERVER` Region `New Region Data`))

(event `On Save Site SERVER`
  (params (Site :type "/CesiumNetBoxVisualization/G2VisualizationActors/NetBoxActors/BP_Netbox_Site Object Reference") (`New Site Data` :type "SiteStruct Structure"))
  ;[1 1 1] Netbox Interface
  (`/CesiumNetBoxVisualization/BP_G2_Topology.On Save Site` (`/CesiumNetBoxVisualization/G2VisualizationActors/BP_G2_Topology_Actor.NetBox Visualization` Site) Site `New Site Data`))

(event `/CesiumNetBoxVisualization/BP_G2_Topology_Pawn_Interface.On Save Site`
  (params (Site :type "/CesiumNetBoxVisualization/G2VisualizationActors/NetBoxActors/BP_Netbox_Site Object Reference") (`New Site Data` :type "SiteStruct Structure"))
  ;[1 1 1] Netbox Interface
  (`self.On Save Site SERVER` Site `New Site Data`))

(event `On Save Location SERVER`
  (params (Location :type "/CesiumNetBoxVisualization/G2VisualizationActors/NetBoxActors/BP_Netbox_Location Object Reference") (`New Location Data` :type "LocationStruct Structure"))
  ;[1 1 1] Netbox Interface
  (`/CesiumNetBoxVisualization/BP_G2_Topology.On Save Location` (`/CesiumNetBoxVisualization/G2VisualizationActors/BP_G2_Topology_Actor.NetBox Visualization` Location) Location `New Location Data`))

(event `/CesiumNetBoxVisualization/BP_G2_Topology_Pawn_Interface.On Save Location`
  (params (Location :type "/CesiumNetBoxVisualization/G2VisualizationActors/NetBoxActors/BP_Netbox_Location Object Reference") (`New Location Data` :type "LocationStruct Structure"))
  ;[1 1 1] Netbox Interface
  (`self.On Save Location SERVER` Location `New Location Data`))

(event `self.ReceiveTick`
  (params (DeltaSeconds :type "Float (single-precision)"))
  (bind _grabbed_netbox_actor (`self.Grabbed Netbox Actor`))
  (bind _grabbed_netbox_actor_2 (`self.Grabbed Netbox Actor`))
  (bind (_worldlocation _worlddirection) (`PlayerController.DeprojectMousePositionToWorld` (`GameplayStatics.GetPlayerController` 0)))
  (bind (_returnvalue_x _returnvalue_y _returnvalue_z) (`KismetMathLibrary.BreakVector` (`CesiumGlobeAnchorComponent.GetLongitudeLatitudeHeight` (`/CesiumNetBoxVisualization/G2VisualizationActors/BP_G2_Topology_Actor.Cesium Globe` _grabbed_netbox_actor_2))))
  (bind _center_of_earth (`/CesiumNetBoxVisualization/BP_G2_Topology.Center of Earth` (`/CesiumNetBoxVisualization/G2VisualizationActors/BP_G2_Topology_Actor.NetBox Visualization` _grabbed_netbox_actor)))
  (bind (_grab_location _valid_location) (`self.Get Grab Location` _worldlocation _worlddirection _center_of_earth (`KismetMathLibrary.Vector_Distance` _center_of_earth (`self.K2_GetActorLocation` _grabbed_netbox_actor))))
  ;[1 1 1] Tick stuff
  (`parent.ReceiveTick` DeltaSeconds)
  (if (and (`self.GrabMode`) (`KismetSystemLibrary.IsValid` (`self.Grabbed Netbox Actor`)))
    (if _valid_location
      (`self.Move G2 Topology Actor SERVER` (`self.Grabbed Netbox Actor`) (`self.Get Transform from Lat Long` (- _grab_location (`self.WorldGrabLocationOffset`)) (`/CesiumNetBoxVisualization/G2VisualizationActors/BP_G2_Topology_Actor.NetBox Visualization` _grabbed_netbox_actor_2) _returnvalue_z)))))

(event `On Save Rack SERVER`
  (params (Rack :type "/CesiumNetBoxVisualization/G2VisualizationActors/NetBoxActors/BP_Netbox_Rack Object Reference") (`New Rack Data` :type "RackStruct Structure"))
  ;[1 1 1] Netbox Interface
  (`/CesiumNetBoxVisualization/BP_G2_Topology.On Save Rack` (`/CesiumNetBoxVisualization/G2VisualizationActors/BP_G2_Topology_Actor.NetBox Visualization` Rack) Rack `New Rack Data`))

(event `/CesiumNetBoxVisualization/BP_G2_Topology_Pawn_Interface.On Save Rack`
  (params (Rack :type "/CesiumNetBoxVisualization/G2VisualizationActors/NetBoxActors/BP_Netbox_Rack Object Reference") (`New Rack Data` :type "RackStruct Structure"))
  ;[1 1 1] Netbox Interface
  (`self.On Save Rack SERVER` Rack `New Rack Data`))

(event `On Save Device SERVER`
  (params (Device :type "/CesiumNetBoxVisualization/G2VisualizationActors/NetBoxActors/BP_Netbox_Device Object Reference") (`New Device Data` :type "DeviceStruct Structure"))
  ;[1 1 1] Netbox Interface
  (`/CesiumNetBoxVisualization/BP_G2_Topology.On Save Device` (`/CesiumNetBoxVisualization/G2VisualizationActors/BP_G2_Topology_Actor.NetBox Visualization` Device) Device `New Device Data`))

(event `/CesiumNetBoxVisualization/BP_G2_Topology_Pawn_Interface.On Save Device`
  (params (Device :type "/CesiumNetBoxVisualization/G2VisualizationActors/NetBoxActors/BP_Netbox_Device Object Reference") (`New Device Data` :type "DeviceStruct Structure"))
  ;[1 1 1] Netbox Interface
  (`self.On Save Device SERVER` Device `New Device Data`))

(fn `CartesianToLatLong`
  (params (Cartesian :type "Vector Structure"))
  (returns (Latitude :type "Float (double-precision)") (Longitude :type "Float (double-precision)"))
  (locals (Lat :type "Float (double-precision)"))
  (bind _returnvalue (`CesiumGeoreference.GetDefaultGeoreference`))
  (bind (_returnvalue_x _returnvalue_y) (`KismetMathLibrary.BreakVector` (`CesiumGeoreference.TransformUnrealToLongitudeLatitudeHeight` _returnvalue Cartesian)))
  (return _returnvalue_y _returnvalue_x))

(fn `FlyToRegion`
  (params (Region :type "/CesiumNetBoxVisualization/G2VisualizationActors/NetBoxActors/BP_Netbox_Region Object Reference"))
  (`self.Fly to New Location Longitude Latitude Height` (`KismetMathLibrary.MakeVector` (`/CesiumNetBoxVisualization/G2VisualizationActors/NetBoxActors/BP_Netbox_Region.Longitude` Region) (`/CesiumNetBoxVisualization/G2VisualizationActors/NetBoxActors/BP_Netbox_Region.Latitude` Region) 10000.0)))

(fn `FlyToSite`
  (params (Site :type "/CesiumNetBoxVisualization/G2VisualizationActors/NetBoxActors/BP_Netbox_Site Object Reference"))
  (`self.Fly to New Location Longitude Latitude Height` (`KismetMathLibrary.MakeVector` (`/CesiumNetBoxVisualization/G2VisualizationActors/NetBoxActors/BP_Netbox_Region.Longitude` Site) (`/CesiumNetBoxVisualization/G2VisualizationActors/NetBoxActors/BP_Netbox_Region.Latitude` Site) 2500.0)))

(fn `Get Grab Location`
  (params (`Click World Location` :type "Vector Structure") (`Click World Direction` :type "Vector Structure") (`Center of Earth Location` :type "Vector Structure") (`Distance from Center of Earth` :type "Float (double-precision)"))
  (returns (`Grab Location` :type "Vector Structure") (`Valid Location` :type Boolean))
  (bind _returnvalue (- `Click World Location` `Center of Earth Location`))
  (bind (_solution_1 _solution_2 _valid_solutions) (`self.Solve Quadratic Formula` (`KismetMathLibrary.Square` (`KismetMathLibrary.VSize` `Click World Direction`)) (* 2.0 (`KismetMathLibrary.Dot_VectorVector` _returnvalue `Click World Direction`)) (- (`KismetMathLibrary.Square` (`KismetMathLibrary.VSize` _returnvalue)) (`KismetMathLibrary.Square` `Distance from Center of Earth`))))
  (return (+ `Click World Location` (* `Click World Direction` (`KismetMathLibrary.FMin` _solution_1 _solution_2))) _valid_solutions))

(fn `Get Transform from Lat Long`
  (params (`Globe Surface Position` :type "Vector Structure") (`NetBox Visualization` :type "NetBoxVisualization Object Reference") (`Original Height` :type "Float (double-precision)"))
  (returns (ReturnValue :type "Transform Structure"))
  (bind _returnvalue (`CesiumGeoreference.GetDefaultGeoreference`))
  (bind (_returnvalue_x _returnvalue_y) (`KismetMathLibrary.BreakVector` (`CesiumGeoreference.TransformUnrealToLongitudeLatitudeHeight` _returnvalue `Globe Surface Position`)))
  (bind _returnvalue_2 (`CesiumGeoreference.TransformLongitudeLatitudeHeightToUnreal` _returnvalue (`KismetMathLibrary.MakeVector` _returnvalue_x _returnvalue_y `Original Height`)))
  (return (`KismetMathLibrary.MakeTransform` _returnvalue_2 (`NetBoxVisualization.GetRotationRelativeToSurface` `NetBox Visualization` _returnvalue_2))))

(fn `Handle Actor Clicked`
  (params (`Clicked Actor` :type "Actor Object Reference") (`Hit Distance` :type "Float (single-precision)") (`Hit Location` :type "Vector Structure"))
  (locals (`Hit Distance ` :type "Float (double-precision)") (`Hit Location Offset` :type "Vector Structure"))
  (set `local.Hit Distance ` `Hit Distance`)
  (set `local.Hit Location Offset` (- `Hit Location` (`self.K2_GetActorLocation` `Clicked Actor`)))
  (bind _asbp_g2_topology_actor (cast `/CesiumNetBoxVisualization/G2VisualizationActors/BP_G2_Topology_Actor` `Clicked Actor`)
    (:`then`
      (switch `/CesiumNetBoxVisualization/G2VisualizationActors/G2TopologyActorClass` (`/CesiumNetBoxVisualization/G2VisualizationActors/BP_G2_Topology_Actor.Get G2 Topology Actor Class` _asbp_g2_topology_actor)
        (:`NewEnumerator0`
          (bind _asbp_netbox_region (cast `/CesiumNetBoxVisualization/G2VisualizationActors/NetBoxActors/BP_Netbox_Region` `Clicked Actor`))
          (`self.Handle Region Clicked` _asbp_netbox_region (`local.Hit Location Offset`) (`local.Hit Distance `)))
        (:`NewEnumerator1`
          (bind _asbp_netbox_site (cast `/CesiumNetBoxVisualization/G2VisualizationActors/NetBoxActors/BP_Netbox_Site` `Clicked Actor`))
          (`self.Handle Site Clicked` _asbp_netbox_site (`local.Hit Location Offset`) (`local.Hit Distance `)))
        (:`NewEnumerator4`
          (bind _asbp_netbox_location (cast `/CesiumNetBoxVisualization/G2VisualizationActors/NetBoxActors/BP_Netbox_Location` `Clicked Actor`))
          (`self.Handle Location Clicked` _asbp_netbox_location (`local.Hit Location Offset`) (`local.Hit Distance `)))
        (:`NewEnumerator6`
          (bind _asbp_netbox_device (cast `/CesiumNetBoxVisualization/G2VisualizationActors/NetBoxActors/BP_Netbox_Device` `Clicked Actor`))
          (`/CesiumNetBoxVisualization/G2VisualizationActors/BP_G2_Topology_Actor.On Pressed` _asbp_netbox_device))
        (:`NewEnumerator7`
          (bind _asbp_g2_node (cast `/CesiumNetBoxVisualization/G2VisualizationActors/BP_G2_Node` `Clicked Actor`))
          (`self.Handle Node Clicked` _asbp_g2_node (`local.Hit Location Offset`) (`local.Hit Distance `)))
        (:`NewEnumerator8`
          (bind _asbp_3d_region_display (cast `/CesiumNetBoxVisualization/G2VisualizationActors/NetBoxActors/BP_3D_Region_Display` `Clicked Actor`))
          (bind _asbp_netbox_region_2 (cast `/CesiumNetBoxVisualization/G2VisualizationActors/NetBoxActors/BP_Netbox_Region` (`self.GetAttachParentActor` _asbp_3d_region_display)))
          (`self.FlyToRegion` _asbp_netbox_region_2))))
    (:`CastFailed`
      (set `self.GrabMode` false))))

(fn `Handle Location Clicked`
  (params (Location :type "/CesiumNetBoxVisualization/G2VisualizationActors/NetBoxActors/BP_Netbox_Location Object Reference") (WorldGrabLocationOffset :type "Vector Structure") (OriginalDistanceToObject :type "Float (double-precision)"))
  (bind _netbox_visualization (`/CesiumNetBoxVisualization/G2VisualizationActors/BP_G2_Topology_Actor.NetBox Visualization` Location))
  (bind _location_data_display (`/CesiumNetBoxVisualization/BP_G2_Topology.Location Data Display` _netbox_visualization))
  (bind _selected_location (`/CesiumNetBoxVisualization/Widgets/LocationWidgets/LocationDataDisplay.Selected Location` _location_data_display))
  (set `self.WorldGrabLocationOffset` WorldGrabLocationOffset)
  (set `self.OriginalDistanceToObject` OriginalDistanceToObject)
  (bind _overlappinglocations (`/CesiumNetBoxVisualization/BP_G2_Topology.GetOverlappingLocations` _netbox_visualization Location))
  (if (and (`Widget.IsVisible` _location_data_display) (`KismetArrayLibrary.Array_Contains` _overlappinglocations _selected_location))
    (`/CesiumNetBoxVisualization/G2VisualizationActors/BP_G2_Topology_Actor.On Selected` _selected_location)
    (set `self.Grabbed Netbox Actor` _selected_location)
    (set `self.GrabMode` true :!label _label)
    (else
      (`/CesiumNetBoxVisualization/G2VisualizationActors/BP_G2_Topology_Actor.On Pressed` Location)
      (if (== (`KismetArrayLibrary.Array_Length` _overlappinglocations) 1)
        (set `self.Grabbed Netbox Actor` Location)
        (goto _label)))))

(fn `Handle Node Clicked`
  (params (Node :type "/CesiumNetBoxVisualization/G2VisualizationActors/BP_G2_Node Object Reference") (WorldGrabLocationOffset :type "Vector Structure") (OriginalDistanceToObject :type "Float (double-precision)"))
  (bind _netbox_visualization (`/CesiumNetBoxVisualization/G2VisualizationActors/BP_G2_Topology_Actor.NetBox Visualization` Node))
  (bind _node_data_display (`/CesiumNetBoxVisualization/BP_G2_Topology.Node Data Display` _netbox_visualization))
  (bind _selected_node (`/CesiumNetBoxVisualization/Widgets/NodeWidgets/NodeDataDisplay.Selected Node` _node_data_display))
  (set `self.WorldGrabLocationOffset` WorldGrabLocationOffset)
  (set `self.OriginalDistanceToObject` OriginalDistanceToObject)
  (bind _overlappingnodes (`/CesiumNetBoxVisualization/BP_G2_Topology.GetOverlappingNodes` _netbox_visualization Node))
  (if (and (`Widget.IsVisible` _node_data_display) (`KismetArrayLibrary.Array_Contains` _overlappingnodes _selected_node))
    (`/CesiumNetBoxVisualization/G2VisualizationActors/BP_G2_Topology_Actor.On Selected` _selected_node)
    (set `self.Grabbed Netbox Actor` _selected_node)
    (set `self.GrabMode` true :!label _label)
    (else
      (`/CesiumNetBoxVisualization/G2VisualizationActors/BP_G2_Topology_Actor.On Pressed` Node)
      (if (== (`KismetArrayLibrary.Array_Length` _overlappingnodes) 1)
        (set `self.Grabbed Netbox Actor` Node)
        (goto _label)))))

(fn `Handle Region Clicked`
  (params (Region :type "/CesiumNetBoxVisualization/G2VisualizationActors/NetBoxActors/BP_Netbox_Region Object Reference") (WorldGrabLocationOffset :type "Vector Structure") (OriginalDistanceToObject :type "Float (double-precision)"))
  (bind _netbox_visualization (`/CesiumNetBoxVisualization/G2VisualizationActors/BP_G2_Topology_Actor.NetBox Visualization` Region))
  (bind _region_data_display (`/CesiumNetBoxVisualization/BP_G2_Topology.Region Data Display` _netbox_visualization))
  (bind _selected_region (`/CesiumNetBoxVisualization/Widgets/RegionWidgets/RegionDataDisplay.Selected Region` _region_data_display))
  (set `self.WorldGrabLocationOffset` WorldGrabLocationOffset)
  (set `self.OriginalDistanceToObject` OriginalDistanceToObject)
  (bind _overlapping_regions (`/CesiumNetBoxVisualization/BP_G2_Topology.GetOverlappingRegions` _netbox_visualization Region))
  (if (and (`Widget.IsVisible` _region_data_display) (`KismetArrayLibrary.Array_Contains` _overlapping_regions _selected_region))
    (`/CesiumNetBoxVisualization/G2VisualizationActors/BP_G2_Topology_Actor.On Selected` _selected_region)
    (set `self.Grabbed Netbox Actor` _selected_region)
    (set `self.GrabMode` true :!label _label)
    (else
      (`/CesiumNetBoxVisualization/G2VisualizationActors/BP_G2_Topology_Actor.On Pressed` Region)
      (if (== (`KismetArrayLibrary.Array_Length` _overlapping_regions) 1)
        (set `self.Grabbed Netbox Actor` Region)
        (goto _label)))))

(fn `Handle Site Clicked`
  (params (Site :type "/CesiumNetBoxVisualization/G2VisualizationActors/NetBoxActors/BP_Netbox_Site Object Reference") (WorldGrabLocationOffset :type "Vector Structure") (OriginalDistanceToObject :type "Float (double-precision)"))
  (bind _netbox_visualization (`/CesiumNetBoxVisualization/G2VisualizationActors/BP_G2_Topology_Actor.NetBox Visualization` Site))
  (bind _site_data_display (`/CesiumNetBoxVisualization/BP_G2_Topology.Site Data Display` _netbox_visualization))
  (bind _selected_site (`/CesiumNetBoxVisualization/Widgets/SiteWidgets/SiteDataDisplay.Selected Site` _site_data_display))
  (set `self.WorldGrabLocationOffset` WorldGrabLocationOffset)
  (set `self.OriginalDistanceToObject` OriginalDistanceToObject)
  (bind _overlappingsites (`/CesiumNetBoxVisualization/BP_G2_Topology.GetOverlappingSites` _netbox_visualization Site))
  (if (and (`Widget.IsVisible` _site_data_display) (`KismetArrayLibrary.Array_Contains` _overlappingsites _selected_site))
    (`/CesiumNetBoxVisualization/G2VisualizationActors/BP_G2_Topology_Actor.On Selected` _selected_site)
    (set `self.Grabbed Netbox Actor` _selected_site)
    (set `self.GrabMode` true :!label _label)
    (else
      (`/CesiumNetBoxVisualization/G2VisualizationActors/BP_G2_Topology_Actor.On Pressed` Site)
      (if (== (`KismetArrayLibrary.Array_Length` _overlappingsites) 1)
        (set `self.Grabbed Netbox Actor` Site)
        (goto _label)))))

(fn `Lat Long to Cartesian`
  (params (Latitude :type "Float (double-precision)") (Longitude :type "Float (double-precision)"))
  (returns (Cartesian :type "Vector Structure"))
  (bind _returnvalue (`CesiumGeoreference.GetDefaultGeoreference`))
  (return (`CesiumGeoreference.TransformLongitudeLatitudeHeightToUnreal` _returnvalue (`KismetMathLibrary.MakeVector` Longitude Latitude 10000.0))))

(fn `Setup Restore Location Widget`
  (bind _returnvalue (`|CreateWidget` "/CesiumNetBoxVisualization/Widgets/RestoreLocationWidget.RestoreLocationWidget_C"))
  (bind _output_get (set `self.Restore Location Widget` _returnvalue))
  (`UserWidget.AddToViewport` _output_get 1)
  (`Widget.SetVisibility` _output_get "SelfHitTestInvisible"))

(fn `Solve Quadratic Formula`
  (params (A :type "Float (double-precision)") (B :type "Float (double-precision)") (C :type "Float (double-precision)"))
  (returns (`Solution 1` :type "Float (double-precision)") (`Solution 2` :type "Float (double-precision)") (`Valid Solutions` :type Boolean))
  (bind _returnvalue (* B -1.0))
  (bind _returnvalue_2 (- (`KismetMathLibrary.Square` B) (* 4.0 A C)))
  (bind _returnvalue_3 (`KismetMathLibrary.Sqrt` _returnvalue_2))
  (if (< _returnvalue_2 0.0)
    (return 0.0 0.0 false)
    (else
      (return (/ (+ _returnvalue _returnvalue_3) 2.0 A) (/ (- _returnvalue _returnvalue_3) 2.0 A) true))))

(fn `Update Node Data Display`
  (params (Node :type "/CesiumNetBoxVisualization/G2VisualizationActors/BP_G2_Node Object Reference") (`New Latitute` :type "Float (double-precision)") (`New Longitude` :type "Float (double-precision)"))
  (bind _node_data_display (`/CesiumNetBoxVisualization/BP_G2_Topology.Node Data Display` (`/CesiumNetBoxVisualization/G2VisualizationActors/BP_G2_Topology_Actor.NetBox Visualization` Node)))
  (if (== Node (`/CesiumNetBoxVisualization/Widgets/NodeWidgets/NodeDataDisplay.Selected Node` _node_data_display))
    (`/CesiumNetBoxVisualization/Widgets/NodeWidgets/NodeDataDisplay.Update Lat Long` _node_data_display `New Latitute` `New Longitude`)))

(fn `Update Region Data Display`
  (params (Region :type "/CesiumNetBoxVisualization/G2VisualizationActors/NetBoxActors/BP_Netbox_Region Object Reference") (`New Latitude` :type "Float (double-precision)") (`New Longitude` :type "Float (double-precision)"))
  (bind _region_data_display (`/CesiumNetBoxVisualization/BP_G2_Topology.Region Data Display` (`/CesiumNetBoxVisualization/G2VisualizationActors/BP_G2_Topology_Actor.NetBox Visualization` Region)))
  (if (== Region (`/CesiumNetBoxVisualization/Widgets/RegionWidgets/RegionDataDisplay.Selected Region` _region_data_display))
    (`/CesiumNetBoxVisualization/Widgets/RegionWidgets/RegionDataDisplay.Update Lat Long` _region_data_display `New Latitude` `New Longitude`)))

(fn `Update Site Data Display`
  (params (Site :type "/CesiumNetBoxVisualization/G2VisualizationActors/NetBoxActors/BP_Netbox_Site Object Reference") (`New Latitute` :type "Float (double-precision)") (`New Longitude` :type "Float (double-precision)"))
  (bind _site_data_display (`/CesiumNetBoxVisualization/BP_G2_Topology.Site Data Display` (`/CesiumNetBoxVisualization/G2VisualizationActors/BP_G2_Topology_Actor.NetBox Visualization` Site)))
  (if (== Site (`/CesiumNetBoxVisualization/Widgets/SiteWidgets/SiteDataDisplay.Selected Site` _site_data_display))
    (`/CesiumNetBoxVisualization/Widgets/SiteWidgets/SiteDataDisplay.Update Lat Long` _site_data_display `New Latitute` `New Longitude`)))

(fn `UserConstructionScript`
  (`parent.UserConstructionScript`))