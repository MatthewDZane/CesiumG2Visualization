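; Base actor for geospatial visualizations on a Cesium globe, providing shared helpers and placeholder functions for child classes.
; Construction stores a Cesium globe anchor root reference, and helper functions range-check latitude and longitude.
; An attach helper parents the actor to the result of GetValidParentActor, keeping relative transforms.
; That lookup, along with color, mesh setup, press, selection and string ID functions, is an empty stub here.
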(fn `Attach to Valid Parent Actor`
  (returns (`Parent Actor` :type "Actor Object Reference"))
  (bind _parent_actor (`self.Get Valid Parent Actor`))
  (`self.K2_AttachToActor` _parent_actor "None" "KeepRelative" "KeepRelative" "KeepRelative")
  (return _parent_actor))

(fn `Get String ID`
  (returns (`String ID` :type String))
  (return ""))

(fn `Get Valid Parent Actor`
  (returns (`Parent Actor` :type "Actor Object Reference"))
  (return null))

(fn `On Pressed`)

(fn `On Selected`)

(fn `Set Color`)

(fn `Setup Static Mesh Component`
  (params (`New Scale` :type "Vector Structure")))

(fn `UserConstructionScript`
  (set `self.Cesium GlobeRoot` (`self.CesiumGlobeAnchorRoot`)))

(fn `Valid Latitude`
  (params (Latitude :type "Float (double-precision)"))
  (returns (Valid :type Boolean))
  (return (`KismetMathLibrary.InRange_FloatFloat` Latitude -90.0 90.0)))

(fn `Valid Latitude Longitude`
  (params (Latitude :type "Float (double-precision)") (Longitude :type "Float (double-precision)"))
  (returns (Valid :type Boolean))
  (return (and (`self.Valid Latitude` Latitude) (`self.Valid Longitude` Longitude))))

(fn `Valid Longitude`
  (params (Longitude :type "Float (double-precision)"))
  (returns (Valid :type Boolean))
  (return (`KismetMathLibrary.InRange_FloatFloat` Longitude -180.0 180.0)))