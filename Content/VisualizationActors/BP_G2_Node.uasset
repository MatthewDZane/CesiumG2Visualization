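; BP_G2_Node is a network node in the NetBox visualization, drawn as a scaled sphere with a dynamic material.
; It can be reassigned between Devices by name and takes latitude/longitude from the Device's Site, using its own values when the site is "TBD".
; Color reflects MTU (9000, other or unknown), and untethered nodes (zero coordinates or non-9000 MTU) glow.
; Press and selection events are forwarded to NetBoxVisualization, which also serves as its parent actor.
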(fn `Change Device`
  (params (NewDeviceName :type String))
  (bind _device (`self.Device`))
  (bind _value (`BlueprintMapLibrary.Map_Find` (`/CesiumNetBoxVisualization/BP_NetBox_Visualization.Name to Device Map` (`self.NetBox Visualization`)) NewDeviceName))
  (`/Engine/EditorBlueprintResources/StandardMacros.IsValid` _device
    (:`Is Valid`
      (`KismetArrayLibrary.Array_RemoveItem` (`/CesiumNetBoxVisualization/VisualizationActors/NetBoxActors/BP_Netbox_Device.Nodes` _device) self))
    (:`Is Not Valid`
      _))
  (set `self.Device` _value)
  (`KismetArrayLibrary.Array_Add` (`/CesiumNetBoxVisualization/VisualizationActors/NetBoxActors/BP_Netbox_Device.Nodes` _value) self))

(fn `Get Latitude`
  (returns (Latitude :type "Float (double-precision)"))
  (bind _site (`/CesiumNetBoxVisualization/VisualizationActors/NetBoxActors/BP_Netbox_Device.Site` (`self.Device`)))
  (if (`KismetStringLibrary.EqualEqual_StrStr` (`/CesiumNetBoxVisualization/VisualizationActors/NetBoxActors/BP_Netbox_Actor.Name` _site) "TBD")
    (return (`self.Latitude`))
    (else
      (return (`/CesiumNetBoxVisualization/VisualizationActors/NetBoxActors/BP_Netbox_Actor.Latitude` _site)))))

(fn `Get Longitude`
  (returns (Longitude :type "Float (double-precision)"))
  (bind _site (`/CesiumNetBoxVisualization/VisualizationActors/NetBoxActors/BP_Netbox_Device.Site` (`self.Device`)))
  (if (`KismetStringLibrary.EqualEqual_StrStr` (`/CesiumNetBoxVisualization/VisualizationActors/NetBoxActors/BP_Netbox_Actor.Name` _site) "TBD")
    (return (`self.Longitude`))
    (else
      (return (`/CesiumNetBoxVisualization/VisualizationActors/NetBoxActors/BP_Netbox_Actor.Longitude` _site)))))

(fn `Get Valid Parent Actor`
  (returns (`Parent Actor` :type "Actor Object Reference"))
  (return (`self.NetBox Visualization`)))

(fn `On Pressed`
  (`/CesiumNetBoxVisualization/BP_NetBox_Visualization.OnNodePressed` (`self.NetBox Visualization`) self))

(fn `On Selected`
  (`/CesiumNetBoxVisualization/BP_NetBox_Visualization.OnNodeSelected` (`self.NetBox Visualization`) self))

(fn `Set Color`
  (bind _mtu (`self.MTU`))
  (bind _dynamic_material (`self.Dynamic Material`))
  ;[1 1 1] Node is green if MTU = 9000, black if other known value, and red if unknown
  (if (== _mtu 9000)
    (`MaterialInstanceDynamic.SetVectorParameterValue` _dynamic_material "Color" (struct :`G` 0.44375 :`B` 0.089353 :`A` 1.0))
    (elif (== _mtu 0)
      (`MaterialInstanceDynamic.SetVectorParameterValue` _dynamic_material "Color" (struct :`R` 0.94375 :`A` 1.0))
      (else
        (`MaterialInstanceDynamic.SetVectorParameterValue` _dynamic_material "Color" (struct :`R` 0.127083 :`G` 0.127083 :`B` 0.127083 :`A` 1.0)))))
  (if (`self.Untethered`)
    (`MaterialInstanceDynamic.SetScalarParameterValue` (`self.Dynamic Material`) "Emissive Color" 3.0) ; untethered nodes are set to "glow"
  )
  (return))

(fn `Setup Static Mesh Component`
  (params (`New Scale` :type "Vector Structure"))
  (bind _returnvalue (`AddComponent|NODE_AddBP_Static_Mesh_Component-1`))
  (`SceneComponent.SetRelativeScale3D` _returnvalue `New Scale`)
  (`StaticMeshComponent.SetStaticMesh` _returnvalue "/Engine/EngineMeshes/Sphere.Sphere")
  (set `self.Static Mesh Component` _returnvalue)
  (bind _returnvalue_2 (`PrimitiveComponent.CreateDynamicMaterialInstance` (`self.Static Mesh Component`) 0 "/CesiumNetBoxVisualization/VisualizationActors/M_Node.M_Node" "None"))
  (set `self.Dynamic Material` _returnvalue_2))

(fn `Untethered`
  (returns (Untethered :type Boolean))
  (return (or (and (== (`self.Get Latitude`) 0.0) (== (`self.Get Longitude`) 0.0)) (!= (`self.MTU`) 9000))))

(fn `UserConstructionScript`)