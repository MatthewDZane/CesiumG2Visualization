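; BP_G2_Link is a visualization actor drawing a curved spline-mesh link between Source and Target actors around a globe center.
; UpdateSpline sets endpoints, rotations and middle tangent, then stretches spline meshes between consecutive points.
; For two-segment splines, the midpoint sits at the endpoints' average radius, plus a distance-scaled height offset unless their angle is below a minimum.
; SetColor tints meshes red or blue by a Delay threshold, despite comments saying green, and applies the given opacity.
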(fn `Get String ID`
  (returns (`String ID` :type String))
  (return (`self.ID`)))

(fn `Get Valid Parent Actor`
  (returns (`Parent Actor` :type "Actor Object Reference"))
  (return (`self.NetBox Visualization`)))

(fn `Set Color `
  (params (`Mesh Opacity` :type "Float (double-precision)" :default 0.8))
  (bind _returnvalue (`KismetMathLibrary.Conv_BoolToDouble` (not (< (`self.Delay`) 10.0))))
  (set `self.MeshColor` (`KismetMathLibrary.Conv_LinearColorToVector` (`KismetMathLibrary.MakeColor` _returnvalue 0.0 (- 1.0 _returnvalue))))
  ;[1 1 1] Update Color and Opacity of Mesh i to i+1
  (for _array_element (`self.Spline Mesh Component I`)
    (`MeshComponent.SetVectorParameterValueOnMaterials` _array_element "Color" (`self.MeshColor`))
    (`MeshComponent.SetScalarParameterValueOnMaterials` _array_element "Opacity" `Mesh Opacity`)))

(fn `Set Spline Mid Point Height`
  (params (`Curve Height` :type "Float (double-precision)") (`Center of Earth` :type "Vector Structure"))
  (bind _spline_component (`self.Spline Component`))
  (bind _returnvalue (- (`self.GetRelativeLocation` (`self.Source`)) `Center of Earth`))
  (bind _returnvalue_2 (- (`self.GetRelativeLocation` (`self.Target`)) `Center of Earth`))
  (bind _returnvalue_3 (- _returnvalue _returnvalue_2))
  (bind _returnvalue_4 (* (`KismetMathLibrary.Normal` (/ (+ _returnvalue _returnvalue_2) 2.0)) (/ (+ (`KismetMathLibrary.VSize` _returnvalue) (`KismetMathLibrary.VSize` _returnvalue_2)) 2.0)))
  (if (< (`self.AngleBetweenVectors` _returnvalue _returnvalue_2) (`self.Min Curve Angel`))
    (`SplineComponent.SetLocationAtSplinePoint` _spline_component 1 (+ `Center of Earth` _returnvalue_4) "Local" true)
    (else
      (`SplineComponent.SetLocationAtSplinePoint` _spline_component 1 (+ `Center of Earth` (+ _returnvalue_4 (* (`KismetMathLibrary.Normal` (`KismetMathLibrary.RotateAngleAxis` (`KismetMathLibrary.Cross_VectorVector` _returnvalue _returnvalue_2) -90.0 _returnvalue_3)) (* `Curve Height` (`KismetMathLibrary.VSize` _returnvalue_3))))) "Local" true))))

(fn `Update Spline Mesh`
  (params (LastIndex :type Integer))
  (locals (`Mesh Color` :type "Vector Structure") (`Mesh Opacity` :type "Float (double-precision)"))
  (bind _spline_component (`self.Spline Component`))
  (for _index (range (+ LastIndex 1))
    (bind _output (`|GetArrayItem` (`self.Spline Mesh Component I`) _index))
    ;[1 1 1] Add Mesh to point i to i+1
    (`SplineMeshComponent.SetForwardAxis` _output "Z" true)
    (bind (_location _tangent) (`SplineComponent.GetLocationAndTangentAtSplinePoint` _spline_component _index "Local"))
    (bind (_location_2 _tangent_2) (`SplineComponent.GetLocationAndTangentAtSplinePoint` _spline_component (+ _index 1) "Local"))
    (`SplineMeshComponent.SetStartAndEnd` _output _location _tangent _location_2 _tangent_2 true)))

(fn `UpdateSpline`
  (params (`Spline Length In` :type Integer) (`Planet Radius In` :type "Float (double-precision)") (`Curve Height In` :type "Float (double-precision)") (`Center of Earth In` :type "Vector Structure"))
  (locals (`Spline Length` :type Integer) (`Start Point` :type "Vector Structure") (Increment :type "Vector Structure") (`Mesh Color` :type "Vector Structure") (`Planet Radius` :type "Float (double-precision)") (`Mesh Opacity` :type "Float (double-precision)") (`Curve Height` :type "Float (double-precision)" :default 0.1) (`Center of Earth` :type "Vector Structure"))
  (bind _spline_component (`self.Spline Component`))
  (bind _spline_length (`local.Spline Length`))
  (bind _spline_length_2 (`local.Spline Length`))
  (bind _spline_component_2 (`self.Spline Component`))
  (bind _relative_location (`self.GetRelativeLocation` (`self.Target`)))
  (bind _relative_location_2 (`self.GetRelativeLocation` (`self.Source`)))
  (bind _returnvalue (- (`SplineComponent.GetLocationAtSplinePoint` _spline_component _spline_length "Local") (`SplineComponent.GetLocationAtSplinePoint` _spline_component 0 "Local")))
  (set `local.Spline Length` `Spline Length In`)
  (set `local.Planet Radius` `Planet Radius In`)
  (set `local.Curve Height` `Curve Height In`)
  (set `local.Center of Earth` `Center of Earth In`)
  (set `local.Start Point` _relative_location_2)
  (set `local.Increment` (/ (- _relative_location _relative_location_2) (`local.Spline Length`)))
  (`SplineComponent.SetLocationAtSplinePoint` _spline_component_2 0 (`local.Start Point`) "Local" true)
  (`SplineComponent.SetLocationAtSplinePoint` _spline_component_2 _spline_length_2 _relative_location "Local" true)
  ;[1 1 1] Update Spline Component
  (if (== _spline_length_2 2)
    (`self.Set Spline Mid Point Height` (`local.Curve Height`) (`local.Center of Earth`)))
  (`SplineComponent.SetRotationAtSplinePoint` _spline_component 0 (`KismetMathLibrary.MakeRotator` 0.0 80.0) "Local" true)
  (`SplineComponent.SetRotationAtSplinePoint` _spline_component (`local.Spline Length`) (`KismetMathLibrary.MakeRotator` 0.0 -80.0) "Local" true)
  (`SplineComponent.SetTangentsAtSplinePoint` _spline_component (/ _spline_length 2) _returnvalue _returnvalue "Local" true)
  (`self.Update Spline Mesh` (- (`local.Spline Length`) 1))
  (return))

(fn `UserConstructionScript`)