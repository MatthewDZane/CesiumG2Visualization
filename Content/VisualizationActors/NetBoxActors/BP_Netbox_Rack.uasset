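; BP_Netbox_Rack is the actor for a NetBox rack in the visualization, reporting selection to NetBoxVisualization.
; It converts to and from rack structs, including world offsets stored as custom fields, and resolves Site and Location through name maps.
; On authority it adds a cabinet mesh chosen by height (42U, otherwise 48U) and depth.
; Devices are placed by U position, and site or location changes update rack lists and reattach the actor.
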(fn `Change Location`
  (params (`Location Name` :type String))
  (bind _location (`self.Location`))
  (bind (_value _returnvalue) (`BlueprintMapLibrary.Map_Find` (`/CesiumNetBoxVisualization/BP_NetBox_Visualization.Name to Location Map` (`self.NetBox Visualization`)) `Location Name`))
  (if (!= (`self.Location`) _value)
    (if _returnvalue
      (`KismetArrayLibrary.Array_Add` (`/CesiumNetBoxVisualization/VisualizationActors/NetBoxActors/BP_Netbox_Location.Racks` _value) self))
    (`/Engine/EditorBlueprintResources/StandardMacros.IsValid` _location
      (:`Is Valid`
        (`KismetArrayLibrary.Array_RemoveItem` (`/CesiumNetBoxVisualization/VisualizationActors/NetBoxActors/BP_Netbox_Location.Racks` _location) self))
      (:`Is Not Valid`
        _))
    (set `self.Location` _value)
    (`self.Attach to Valid Parent Actor`)))

(fn `Change Site`
  (params (`Site Name` :type String))
  (bind _site (`self.Site`))
  (bind (_value _returnvalue) (`BlueprintMapLibrary.Map_Find` (`/CesiumNetBoxVisualization/BP_NetBox_Visualization.Name to Site Map` (`self.NetBox Visualization`)) `Site Name`))
  (if (and (!= (`self.Site`) _value) _returnvalue)
    (`KismetArrayLibrary.Array_Add` (`/CesiumNetBoxVisualization/VisualizationActors/NetBoxActors/BP_Netbox_Site.Racks` _value) self)
    (`/Engine/EditorBlueprintResources/StandardMacros.IsValid` _site
      (:`Is Valid`
        (`KismetArrayLibrary.Array_RemoveItem` (`/CesiumNetBoxVisualization/VisualizationActors/NetBoxActors/BP_Netbox_Site.Racks` _site) self))
      (:`Is Not Valid`
        _))
    (set `self.Site` _value)
    (`self.Attach to Valid Parent Actor`)))

(fn `Get Valid Parent Actor`
  (returns (`Parent Actor` :type "Actor Object Reference"))
  (bind _location (`self.Location`))
  (`/Engine/EditorBlueprintResources/StandardMacros.IsValid` _location
    (:`Is Valid`
      (return _location))
    (:`Is Not Valid`
      (return (`self.Site`)))))

(fn `Insert Device`
  (params (Device :type "/CesiumNetBoxVisualization/VisualizationActors/NetBoxActors/BP_Netbox_Device Object Reference"))
  (`self.SetOwner` Device self)
  (`self.K2_SetActorTransform` (`local.Device`) (`KismetMathLibrary.ComposeTransforms` (`self.GetTransform`) (`KismetMathLibrary.MakeTransform` (`KismetMathLibrary.MakeVector` 0.0 0.0 (* (`KismetMathLibrary.Conv_IntToDouble` (- (`/CesiumNetBoxVisualization/VisualizationActors/NetBoxActors/BP_Netbox_Device.Position` Device) 1)) (`self.Device Offset`))))) false true))

(fn `On Selected`
  (`/CesiumNetBoxVisualization/BP_NetBox_Visualization.OnRackSelected` (`self.NetBox Visualization`) self))

(fn `Setup Static Mesh Component`
  (params (`New Scale` :type "Vector Structure"))
  (bind _outer_depth (`self.Outer Depth`))
  (bind _outer_depth_2 (`self.Outer Depth`))
  (`/Engine/EditorBlueprintResources/ActorMacros.Switch Has Authority`
    (:`Authority`
      (bind _returnvalue (`|AddComponentByClass` "/CesiumNetBoxVisualization/BP_Static_Mesh_Component.BP_Static_Mesh_Component_C"))
      (`SceneComponent.SetRelativeScale3D` _returnvalue `New Scale`)
      (set `self.Static Mesh Component` _returnvalue)
      (if (== (`self.U Height`) 42)
        (if (== _outer_depth_2 36)
          (`StaticMeshComponent.SetStaticMesh` (`self.Static Mesh Component`) "/CesiumNetBoxVisualization/VisualizationActors/NetBoxActors/RackModels/42UFullCab24wx36dx70h.42UFullCab24wx36dx70h")
          (elif (== _outer_depth_2 42)
            (`StaticMeshComponent.SetStaticMesh` (`self.Static Mesh Component`) "/CesiumNetBoxVisualization/VisualizationActors/NetBoxActors/RackModels/42UFullCab24wx42dx70h.42UFullCab24wx42dx70h")
            (else
              (`StaticMeshComponent.SetStaticMesh` (`self.Static Mesh Component`) "/CesiumNetBoxVisualization/VisualizationActors/NetBoxActors/RackModels/42UFullCab24wx50dx70h.42UFullCab24wx50dx70h"))))
        (elif (== _outer_depth 36)
          (`StaticMeshComponent.SetStaticMesh` (`self.Static Mesh Component`) "/CesiumNetBoxVisualization/VisualizationActors/NetBoxActors/RackModels/48UFullCab24wx36dx90_5h.48UFullCab24wx36dx90_5h")
          (elif (== _outer_depth 42)
            (`StaticMeshComponent.SetStaticMesh` (`self.Static Mesh Component`) "/CesiumNetBoxVisualization/VisualizationActors/NetBoxActors/RackModels/48UFullCab24wx42dx90_5h.48UFullCab24wx42dx90_5h")
            (else
              (`StaticMeshComponent.SetStaticMesh` (`self.Static Mesh Component`) "/CesiumNetBoxVisualization/VisualizationActors/NetBoxActors/RackModels/48UFullCab24wx50dx90_5h.48UFullCab24wx50dx90_5h"))))))))

(fn `To Struct`
  (returns (Struct :type "RackStruct Structure"))
  (locals (`Out Struct` :type "RackStruct Structure"))
  (bind _location (`self.Location`))
  (bind _site (`self.Site`))
  (set `local.Out Struct` (make `RackStruct` :`Id` (`self.Id`) :`Url` (`self.Url`) :`Display` (`self.Display`) :`Name` (`self.Name`) :`Custom_fields` (make `CustomRackFields` 0.0 0.0 (`KismetStringLibrary.Conv_VectorToString` (`self.World Location Offset`)) (`KismetStringLibrary.Conv_RotatorToString` (`self.World Rotator Offset`)))))
  (if (`KismetSystemLibrary.IsValid` _site)
    (setmembers `RackStruct` :`StructRef` (`local.Out Struct`) :`Site` (make `RackSite` (`/CesiumNetBoxVisualization/VisualizationActors/NetBoxActors/BP_Netbox_Actor.Id` _site) (`/CesiumNetBoxVisualization/VisualizationActors/NetBoxActors/BP_Netbox_Actor.Url` _site) (`/CesiumNetBoxVisualization/VisualizationActors/NetBoxActors/BP_Netbox_Actor.Display` _site) (`/CesiumNetBoxVisualization/VisualizationActors/NetBoxActors/BP_Netbox_Actor.Name` _site) (`/CesiumNetBoxVisualization/VisualizationActors/NetBoxActors/BP_Netbox_Site.Slug` _site))))
  (if (`KismetSystemLibrary.IsValid` _location)
    (setmembers `RackStruct` :`StructRef` (`local.Out Struct`) :`Location` (make `RackLocation` (`/CesiumNetBoxVisualization/VisualizationActors/NetBoxActors/BP_Netbox_Actor.Id` _location) (`/CesiumNetBoxVisualization/VisualizationActors/NetBoxActors/BP_Netbox_Actor.Url` _location) (`/CesiumNetBoxVisualization/VisualizationActors/NetBoxActors/BP_Netbox_Actor.Display` _location) (`/CesiumNetBoxVisualization/VisualizationActors/NetBoxActors/BP_Netbox_Actor.Name` _location) (`/CesiumNetBoxVisualization/VisualizationActors/NetBoxActors/BP_Netbox_Location.Slug` _location))))
  (return (`local.Out Struct`)))

(fn `Update Data`
  (params (`New Data` :type "RackStruct Structure"))
  (locals (NewLocalVar_0 :type "RackLocation Structure"))
  (bind (_id _url _display _name _facility_id _site _location) (break `RackStruct` `New Data`))
  (bind (_id_2 _url_2 _display_2 _name_2 _facility_id_2 _site_2 _location_2 _tenant _status _role _serial _asset_tag _type _width _u_height _desc_units _outer_width _outer_depth _outer_unit _comments _tags _custom_fields) (break `RackStruct` `New Data`))
  (bind _netbox_visualization (`self.NetBox Visualization`))
  (bind (_rack_latitude _rack_longitude _rack_world_location_offset _rack_world_rotation_offset) (break `CustomRackFields` _custom_fields))
  (set `self.Site` (`BlueprintMapLibrary.Map_Find` (`/CesiumNetBoxVisualization/BP_NetBox_Visualization.Name to Site Map` _netbox_visualization) (`.Name` (break `RackSite` _site))))
  (set `self.Location` (`BlueprintMapLibrary.Map_Find` (`/CesiumNetBoxVisualization/BP_NetBox_Visualization.Name to Location Map` _netbox_visualization) (`.Name` (break `RackLocation` _location))))
  (set `self.Id` _id_2)
  (set `self.Url` _url_2)
  (set `self.Display` _display_2)
  (set `self.Name` _name_2)
  (set `self.World Location Offset` (`KismetStringLibrary.Conv_StringToVector` _rack_world_location_offset))
  (set `self.World Rotator Offset` (`KismetStringLibrary.Conv_StringToRotator` _rack_world_rotation_offset)))

(fn `UserConstructionScript`)