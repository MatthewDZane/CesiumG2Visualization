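; BP_Netbox_Actor is a NetBox visualization actor that carries a latitude and longitude.
; Getters expose both coordinates, and Location Set treats the position as set when either value is non-zero.
; On Move accepts new coordinates but is an empty stub here, and the event graph and construction script add no logic of their own.
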(fn `Get Latitude`
  (returns (Latitude :type "Float (double-precision)"))
  (return (`self.Latitude`)))

(fn `Get Longitude`
  (returns (Longitude :type "Float (double-precision)"))
  (return (`self.Longitude`)))

(fn `Location Set`
  (returns (Set :type Boolean))
  (return (or (!= (`self.Latitude`) 0.0) (!= (`self.Longitude`) 0.0))))

(fn `On Move`
  (params (`New Latitude` :type "Float (double-precision)") (`New Longitude` :type "Float (double-precision)")))

(fn `UserConstructionScript`
  (`parent.UserConstructionScript`))