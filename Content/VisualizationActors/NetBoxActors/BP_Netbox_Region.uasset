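; Actor representing a NetBox region in the visualization, holding its record data, parent link and sites.
; UpdateData and ToStruct convert to and from the region struct, resolving parents through the NetBoxVisualization name map, while ChangeParent re-links child lists.
; It builds a ring mesh colored orange or grey by site presence and attaches a 3D widget display, refreshed after logo download.
; Press and selection events forward to NetBoxVisualization.
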(event `self.ReceiveBeginPlay`)

(event `On Download Logo`
  (bind _logo_url (`self.Logo Url`))
  (if (not (`KismetStringLibrary.IsEmpty` _logo_url))
    (bind _texture (`AsyncTaskDownloadImage.DownloadImage` _logo_url)
      (:`OnSuccess`
        (set `self.Logo` _texture)
        (`KismetSystemLibrary.PrintString` (`KismetStringLibrary.Concat_StrStr` "Image Downloaded Successfully: " _logo_url))
        (bind _asregion_display (cast `/CesiumNetBoxVisualization/Widgets/RegionWidgets/RegionDisplay` (`WidgetComponent.GetUserWidgetObject` (`/CesiumNetBoxVisualization/VisualizationActors/NetBoxActors/BP_3D_Region_Display.Region Display` (`self.3D Display`)))))
        (message `/CesiumNetBoxVisualization/Widgets/DataDisplay.Update Info` _asregion_display))
      (:`OnFail`
        (`KismetSystemLibrary.PrintString` (`KismetStringLibrary.Concat_StrStr` "Image Url was invalid:" _logo_url))))))

(fn `Change Parent`
  (params (`Parent Name` :type String))
  (bind _parent (`self.Parent`))
  (bind (_value _returnvalue) (`BlueprintMapLibrary.Map_Find` (`/CesiumNetBoxVisualization/BP_NetBox_Visualization.Name to Region Map` (`self.NetBox Visualization`)) `Parent Name`))
  (if (!= (`self.Parent`) _value)
    (if _returnvalue
      (`KismetArrayLibrary.Array_Add` (`/Game/VisualizationActors/NetBoxActors/BP_Netbox_Region.Regions` _value) self))
    (`/Engine/EditorBlueprintResources/StandardMacros.IsValid` _parent
      (:`Is Valid`
        (`KismetArrayLibrary.Array_RemoveItem` (`/Game/VisualizationActors/NetBoxActors/BP_Netbox_Region.Regions` _parent) self))
      (:`Is Not Valid`
        _))
    (set `self.Parent` _value)))

(fn `Get Valid Parent Actor`
  (returns (`Parent Actor` :type "Actor Object Reference"))
  (return (`self.NetBox Visualization`)))

(fn `On Pressed`
  (`/CesiumNetBoxVisualization/BP_NetBox_Visualization.OnRegionPressed` (`self.NetBox Visualization`) self))

(fn `On Selected`
  (`/CesiumNetBoxVisualization/BP_NetBox_Visualization.OnRegionSelected` (`self.NetBox Visualization`) self))

(fn `Set Color`
  (bind _dynamic_material (`self.Dynamic Material`))
  (if (> (`KismetArrayLibrary.Array_Length` (`self.Sites`)) 0)
    (`MaterialInstanceDynamic.SetVectorParameterValue` _dynamic_material "Color" (struct :`R` 1.0 :`G` 0.312223 :`A` 1.0))
    (else
      (`MaterialInstanceDynamic.SetVectorParameterValue` _dynamic_material "Color" (struct :`R` 0.234375 :`G` 0.234375 :`B` 0.234375 :`A` 1.0)))))

(fn `Setup 3D Display`
  (params (`Small Setting` :type Boolean))
  (bind _returnvalue (`|SpawnActorFromClass` "/CesiumNetBoxVisualization/VisualizationActors/NetBoxActors/BP_3D_Region_Display.BP_3D_Region_Display_C" (`KismetMathLibrary.MakeTransform` (0.0 0.0 0.0)) "Undefined" "OverrideRootScale" null `Small Setting` null))
  (bind _output_get (set `self.3D Display` _returnvalue))
  (`self.K2_AttachToActor` _output_get self "None" "KeepRelative" "KeepRelative" "KeepRelative" true)
  (bind _asregion_display (cast `/CesiumNetBoxVisualization/Widgets/RegionWidgets/RegionDisplay` (`WidgetComponent.GetUserWidgetObject` (`/CesiumNetBoxVisualization/VisualizationActors/NetBoxActors/BP_3D_Region_Display.Region Display` (`self.3D Display`)))))
  (message `/CesiumNetBoxVisualization/Widgets/DataDisplay.Set Info` _asregion_display self))

(fn `Setup Static Mesh Component`
  (params (`New Scale` :type "Vector Structure"))
  (bind _returnvalue (`AddComponent|NODE_AddStaticMeshComponent-0`))
  (`SceneComponent.SetRelativeScale3D` _returnvalue `New Scale`)
  (`StaticMeshComponent.SetStaticMesh` _returnvalue "/CesiumNetBoxVisualization/VisualizationActors/NetBoxActors/RingMesh.RingMesh")
  (bind _output_get (set `self.Static Mesh Component` _returnvalue))
  (bind _returnvalue_2 (`PrimitiveComponent.CreateDynamicMaterialInstance` _output_get 0 "/CesiumNetBoxVisualization/VisualizationActors/NetBoxActors/M_Region.M_Region" "None"))
  (set `self.Dynamic Material` _returnvalue_2))

(fn `ToStruct`
  (returns (`Region Data` :type "RegionStruct Structure"))
  (bind _regionstruct (make `RegionStruct` :`Id` (`self.Id`) :`Url` (`self.Url`) :`Display` (`self.Display`) :`Name` (`self.Name`) :`Slug` (`self.Slug`) :`Description` (`self.Description`) :`Custom_fields` (make `CustomRegionFields` (`self.Logo Url`) (`KismetStringLibrary.Conv_DoubleToString` (`self.Latitude`)) (`KismetStringLibrary.Conv_DoubleToString` (`self.Longitude`))) :`Site_count` (`KismetArrayLibrary.Array_Length` (`self.Sites`))))
  (if (== (`self.Parent`) null)
    (return _regionstruct)
    (else
      (bind _structout (setmembers `RegionStruct` :`StructRef` _regionstruct :`Parent` (make `RegionParent` (`KismetStringLibrary.Conv_IntToString` (`self.Id`)) (`self.Url`) (`self.Display`) (`self.Name`) (`/Game/VisualizationActors/NetBoxActors/BP_Netbox_Region.Slug` (`self.Parent`)) 1)))
      (return _structout))))

(fn `Update Data`
  (params (`New Data` :type "RegionStruct Structure"))
  (bind (_id _url _display _name _slug _parent _description _tags _custom_fields) (break `RegionStruct` `New Data`))
  (bind (_logo _region_latitude _region_longitude) (break `CustomRegionFields` _custom_fields))
  (set `self.Parent` (`BlueprintMapLibrary.Map_Find` (`/CesiumNetBoxVisualization/BP_NetBox_Visualization.Name to Region Map` (`self.NetBox Visualization`)) (`.Name` (break `RegionParent` (`.Parent` (break `RegionStruct` `New Data`))))))
  (set `self.Id` _id)
  (set `self.Url` _url)
  (set `self.Display` _display)
  (set `self.Name` _name)
  (set `self.Slug` _slug)
  (set `self.Description` _description)
  (set `self.Logo Url` _logo)
  (set `self.Latitude` (`KismetStringLibrary.Conv_StringToDouble` _region_latitude))
  (set `self.Longitude` (`KismetStringLibrary.Conv_StringToDouble` _region_longitude)))

(fn `UserConstructionScript`)