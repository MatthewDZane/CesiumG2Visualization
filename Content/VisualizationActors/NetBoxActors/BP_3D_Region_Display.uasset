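; BP_3D_Region_Display is an actor that shows a RegionDisplay widget in 3D, billboarded toward the viewer.
; Each Tick turns it to face the view and scales it with distance to keep it readable.
; With SmallSetting, it follows the player camera manager and shifts its relative height by distance.
; Otherwise it follows DynamicPawn, using the Cesium georeference to hold it above its Region at a height mapped from pawn altitude.
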(event `self.ReceiveBeginPlay`)

(event `self.ReceiveTick`
  (params (DeltaSeconds :type "Float (single-precision)"))
  (bind _returnvalue (`GameplayStatics.GetPlayerCameraManager` 0))
  (bind _returnvalue_2 (`GameplayStatics.GetPlayerPawn` 0))
  (bind _transformcomponent (`PlayerCameraManager.TransformComponent` _returnvalue))
  (bind _returnvalue_3 (- (`self.K2_GetActorLocation` _returnvalue_2) (`SceneComponent.K2_GetComponentLocation` (`self.Region Display`))))
  (bind _returnvalue_4 (- (`self.K2_GetActorLocation` _returnvalue) (`SceneComponent.K2_GetComponentLocation` (`self.Region Display`))))
  (bind (_returnvalue_x _returnvalue_y _returnvalue_z) (`KismetMathLibrary.BreakVector` (`CesiumGlobeAnchorComponent.GetLongitudeLatitudeHeight` (`GlobeAwareDefaultPawn.GlobeAnchor` (cast `/CesiumForUnreal/DynamicPawn` (`GameplayStatics.GetPlayerPawn` 0) :!pure true)))))
  (bind _returnvalue_5 (`KismetMathLibrary.VSize` _returnvalue_4))
  (if (`self.Small Setting`)
    (`self.K2_SetActorRotation` (`KismetMathLibrary.MakeRotationFromAxes` _returnvalue_4 (`KismetMathLibrary.NegateVector` (`SceneComponent.GetRightVector` _transformcomponent)) (`SceneComponent.GetUpVector` _transformcomponent)))
    (`self.SetActorScale3D` (`KismetMathLibrary.Conv_DoubleToVector` (`KismetMathLibrary.MapRangeClamped` _returnvalue_5 0.0 500.0 0.005 0.05)))
    (`SceneComponent.K2_SetRelativeLocation` (`self.DefaultSceneRoot`) (`KismetMathLibrary.MakeVector` 0.0 0.0 (* (`KismetMathLibrary.MapRangeClamped` _returnvalue_5 0.0 500.0 10.0 50.0) -1.0)) false false)
    (else
      (bind _asdynamic_pawn (cast `/CesiumForUnreal/DynamicPawn` _returnvalue_2))
      (bind _camera (`/CesiumForUnreal/DynamicPawn.Camera` _asdynamic_pawn))
      (`self.K2_SetActorRotation` (`KismetMathLibrary.MakeRotationFromAxes` _returnvalue_3 (`KismetMathLibrary.NegateVector` (`SceneComponent.GetRightVector` _camera)) (`SceneComponent.GetUpVector` _camera)))
      (`self.SetActorScale3D` (`KismetMathLibrary.Conv_DoubleToVector` (`KismetMathLibrary.MapRangeClamped` (`KismetMathLibrary.VSize` _returnvalue_3) 0.0 80000000.0 1.0 30000.0)))
      (bind _asregion_display (cast `/CesiumNetBoxVisualization/Widgets/RegionWidgets/RegionDisplay` (`WidgetComponent.GetWidget` (`self.Region Display`))))
      (bind _returnvalue_6 (`CesiumGeoreference.GetDefaultGeoreference`))
      (bind (_returnvalue_x_2 _returnvalue_y_2) (`KismetMathLibrary.BreakVector` (`CesiumGeoreference.TransformUnrealToLongitudeLatitudeHeight` _returnvalue_6 (`SceneComponent.K2_GetComponentLocation` (`/CesiumNetBoxVisualization/VisualizationActors/BP_Visualization_Actor.DefaultSceneRoot` (`/CesiumNetBoxVisualization/Widgets/RegionWidgets/RegionDisplay.Region` _asregion_display))))))
      (`SceneComponent.K2_SetWorldLocation` (`self.DefaultSceneRoot`) (`CesiumGeoreference.TransformLongitudeLatitudeHeightToUnreal` _returnvalue_6 (`KismetMathLibrary.MakeVector` _returnvalue_x_2 _returnvalue_y_2 (`KismetMathLibrary.MapRangeClamped` _returnvalue_z 100.0 1500000.0 40000.0 500000.0))) false false))))

(fn `UserConstructionScript`)